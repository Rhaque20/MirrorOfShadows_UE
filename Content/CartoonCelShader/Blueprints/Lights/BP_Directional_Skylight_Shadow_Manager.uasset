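; Manager actor that feeds sun, moon and skylight values into MPC_DirectionalAndSkylight for cel-shading materials, updated each tick and on construction.
; Four optional orthographic scene captures follow the player along the sun's direction as shadow-map LODs, publishing position and width.
; An optional simple shadow traces from the player toward sun, or moon when the sun is down, smoothing the result into the collection.
; It can also yaw the sun over time.
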(event `Update Light`
  (bind _directional_light_sun (`self.Directional Light Sun`))
  (bind _directional_light_moon (`self.Directional Light Moon`))
  (bind _skylight (`self.Skylight`))
  (bind _lightcomponent (`Light.LightComponent` _directional_light_moon))
  (bind _lightcomponent_2 (`Light.LightComponent` _directional_light_sun))
  (bind _lightcomponent_3 (`SkyLight.LightComponent` _skylight))
  (bind (_returnvalue_x _returnvalue_y _returnvalue_z) (`KismetMathLibrary.BreakVector` (* (`SceneComponent.GetForwardVector` _lightcomponent) 1)))
  (bind (_returnvalue_x_2 _returnvalue_y_2 _returnvalue_z_2) (`KismetMathLibrary.BreakVector` (* (`SceneComponent.GetForwardVector` _lightcomponent_2) 1)))
  ;[1 1 1] Directional and Skylights
  (`|ExecutionSequence`
    (:`then_0`
      (`/Engine/EditorBlueprintResources/StandardMacros.IsValid` _directional_light_sun
        (:`Is Valid`
          (`KismetMaterialLibrary.SetScalarParameterValue` "/Game/CartoonCelShader/Materials/MaterialCollections/MPC_DirectionalAndSkylight.MPC_DirectionalAndSkylight" "Directional Light Sun Intensity" (`LightComponentBase.Intensity` _lightcomponent_2))
          (if (not true)
            (`LightComponent.SetLightColor` :`self` _lightcomponent_2))
          (`KismetMaterialLibrary.SetVectorParameterValue` "/Game/CartoonCelShader/Materials/MaterialCollections/MPC_DirectionalAndSkylight.MPC_DirectionalAndSkylight" "Directional Light Sun Color" (`LightComponentBase.GetLightColor` _lightcomponent_2))
          (`KismetMaterialLibrary.SetVectorParameterValue` "/Game/CartoonCelShader/Materials/MaterialCollections/MPC_DirectionalAndSkylight.MPC_DirectionalAndSkylight" "Directional Light Sun Vector" (make `LinearColor` _returnvalue_x_2 _returnvalue_y_2 _returnvalue_z_2 1.0))
          (`KismetMaterialLibrary.SetVectorParameterValue` "/Game/CartoonCelShader/Materials/MaterialCollections/MPC_DirectionalAndSkylight.MPC_DirectionalAndSkylight" "Directional Light Sun Right Vector" (`KismetMathLibrary.Conv_VectorToLinearColor` (`SceneComponent.GetRightVector` _lightcomponent_2))))
        (:`Is Not Valid`
          (`KismetSystemLibrary.PrintString` "Set the directional light sun parameter! " true true (struct :`G` 0.66 :`B` 1.0 :`A` 1.0) 1.0))))
    (:`then_1`
      (`/Engine/EditorBlueprintResources/StandardMacros.IsValid` _directional_light_moon
        (:`Is Valid`
          (`KismetMaterialLibrary.SetScalarParameterValue` "/Game/CartoonCelShader/Materials/MaterialCollections/MPC_DirectionalAndSkylight.MPC_DirectionalAndSkylight" "Directional Light Moon Intensity" (`LightComponentBase.Intensity` _lightcomponent))
          (`KismetMaterialLibrary.SetVectorParameterValue` "/Game/CartoonCelShader/Materials/MaterialCollections/MPC_DirectionalAndSkylight.MPC_DirectionalAndSkylight" "Directional Light Moon Color" (`LightComponentBase.GetLightColor` _lightcomponent))
          (`KismetMaterialLibrary.SetVectorParameterValue` "/Game/CartoonCelShader/Materials/MaterialCollections/MPC_DirectionalAndSkylight.MPC_DirectionalAndSkylight" "Directional Light Moon Vector" (make `LinearColor` _returnvalue_x _returnvalue_y _returnvalue_z 1.0))
          (`KismetMaterialLibrary.SetVectorParameterValue` "/Game/CartoonCelShader/Materials/MaterialCollections/MPC_DirectionalAndSkylight.MPC_DirectionalAndSkylight" "Directional Light Moon Right Vector" (`KismetMathLibrary.Conv_VectorToLinearColor` (`SceneComponent.GetRightVector` _lightcomponent))))))
    (:`then_2`
      (`/Engine/EditorBlueprintResources/StandardMacros.IsValid` _skylight
        (:`Is Valid`
          (`KismetMaterialLibrary.SetScalarParameterValue` "/Game/CartoonCelShader/Materials/MaterialCollections/MPC_DirectionalAndSkylight.MPC_DirectionalAndSkylight" "Skylight Intensity" (`LightComponentBase.Intensity` _lightcomponent_3))
          (`KismetMaterialLibrary.SetVectorParameterValue` "/Game/CartoonCelShader/Materials/MaterialCollections/MPC_DirectionalAndSkylight.MPC_DirectionalAndSkylight" "Skylight Color" (`LightComponentBase.GetLightColor` _lightcomponent_3)))))))

(event `Bake Shadowmap`
  (bind _scenecapture_environment_lod0 (`self.SceneCapture_Environment_LOD0`))
  (bind _scenecapture_environment_lod1 (`self.SceneCapture_Environment_LOD1`))
  (bind _scenecapture_environment_lod2 (`self.SceneCapture_Environment_LOD2`))
  (bind _scenecapture_environment_lod3 (`self.SceneCapture_Environment_LOD3`))
  (bind _returnvalue (`self.K2_GetActorLocation` (`GameplayStatics.GetPlayerPawn` 0)))
  (bind _returnvalue_2 (`SceneComponent.K2_GetComponentRotation` (`Light.LightComponent` (`self.Directional Light Sun`))))
  ;[1 1 1] Shadow Map
  (`|ExecutionSequence`
    (:`then_0`
      (if (`self.Shadow 01?`)
        (`SceneComponent.K2_SetWorldRotation` _scenecapture_environment_lod0 _returnvalue_2 false false)
        (`SceneComponent.K2_SetWorldLocation` _scenecapture_environment_lod0 _returnvalue false false)
        (`SceneComponent.K2_AddLocalOffset` _scenecapture_environment_lod0 (-5000.0 0.0 0.0) false false)
        (bind _output_get (set `SceneCaptureComponent2D.OrthoWidth` (`self.Ortho Width LOD0`) _scenecapture_environment_lod0))
        (`KismetMaterialLibrary.SetVectorParameterValue` "/Game/CartoonCelShader/Materials/MaterialCollections/MPC_DirectionalAndSkylight.MPC_DirectionalAndSkylight" "Sun Camera Position LOD0" (`KismetMathLibrary.Conv_VectorToLinearColor` (`SceneComponent.K2_GetComponentLocation` _scenecapture_environment_lod0)))
        (`KismetMaterialLibrary.SetScalarParameterValue` "/Game/CartoonCelShader/Materials/MaterialCollections/MPC_DirectionalAndSkylight.MPC_DirectionalAndSkylight" "Ortho Width LOD0" _output_get)
        (else
          (`SceneComponent.SetVisibility` (`self.SceneCapture_Environment_LOD0`) false false))))
    (:`then_1`
      (if (`self.Shadow 02?`)
        (`SceneComponent.K2_SetWorldRotation` _scenecapture_environment_lod1 _returnvalue_2 false false)
        (`SceneComponent.K2_SetWorldLocation` _scenecapture_environment_lod1 _returnvalue false false)
        (`SceneComponent.K2_AddLocalOffset` _scenecapture_environment_lod1 (-15000.0 0.0 0.0) false false)
        (bind _output_get_2 (set `SceneCaptureComponent2D.OrthoWidth` (`self.Ortho Width LOD1`) _scenecapture_environment_lod1))
        (`KismetMaterialLibrary.SetVectorParameterValue` "/Game/CartoonCelShader/Materials/MaterialCollections/MPC_DirectionalAndSkylight.MPC_DirectionalAndSkylight" "Sun Camera Position LOD1" (`KismetMathLibrary.Conv_VectorToLinearColor` (`SceneComponent.K2_GetComponentLocation` _scenecapture_environment_lod1)))
        (`KismetMaterialLibrary.SetScalarParameterValue` "/Game/CartoonCelShader/Materials/MaterialCollections/MPC_DirectionalAndSkylight.MPC_DirectionalAndSkylight" "Ortho Width LOD1" _output_get_2)
        (else
          (`SceneComponent.SetVisibility` (`self.SceneCapture_Environment_LOD1`) false false))))
    (:`then_2`
      (if (`self.Shadow 03?`)
        (`SceneComponent.K2_SetWorldRotation` _scenecapture_environment_lod2 _returnvalue_2 false false)
        (`SceneComponent.K2_SetWorldLocation` _scenecapture_environment_lod2 _returnvalue false false)
        (`SceneComponent.K2_AddLocalOffset` _scenecapture_environment_lod2 (-15000.0 0.0 0.0) false false)
        (bind _output_get_3 (set `SceneCaptureComponent2D.OrthoWidth` (`self.Ortho Width LOD2`) _scenecapture_environment_lod2))
        (`KismetMaterialLibrary.SetVectorParameterValue` "/Game/CartoonCelShader/Materials/MaterialCollections/MPC_DirectionalAndSkylight.MPC_DirectionalAndSkylight" "Sun Camera Position LOD2" (`KismetMathLibrary.Conv_VectorToLinearColor` (`SceneComponent.K2_GetComponentLocation` _scenecapture_environment_lod2)))
        (`KismetMaterialLibrary.SetScalarParameterValue` "/Game/CartoonCelShader/Materials/MaterialCollections/MPC_DirectionalAndSkylight.MPC_DirectionalAndSkylight" "Ortho Width LOD2" _output_get_3)
        (else
          (`SceneComponent.SetVisibility` (`self.SceneCapture_Environment_LOD2`) false false))))
    (:`then_3`
      (if (`self.Shadow 04?`)
        (`SceneComponent.K2_SetWorldRotation` _scenecapture_environment_lod3 _returnvalue_2 false false)
        (`SceneComponent.K2_SetWorldLocation` _scenecapture_environment_lod3 _returnvalue false false)
        (`SceneComponent.K2_AddLocalOffset` _scenecapture_environment_lod3 (-15000.0 0.0 0.0) false false)
        (bind _output_get_4 (set `SceneCaptureComponent2D.OrthoWidth` (`self.Ortho Width LOD3`) _scenecapture_environment_lod3))
        (`KismetMaterialLibrary.SetVectorParameterValue` "/Game/CartoonCelShader/Materials/MaterialCollections/MPC_DirectionalAndSkylight.MPC_DirectionalAndSkylight" "Sun Camera Position LOD3" (`KismetMathLibrary.Conv_VectorToLinearColor` (`SceneComponent.K2_GetComponentLocation` _scenecapture_environment_lod3)))
        (`KismetMaterialLibrary.SetScalarParameterValue` "/Game/CartoonCelShader/Materials/MaterialCollections/MPC_DirectionalAndSkylight.MPC_DirectionalAndSkylight" "Ortho Width LOD3" _output_get_4)
        (else
          (`SceneComponent.SetVisibility` (`self.SceneCapture_Environment_LOD3`) false false))))))

(event `self.ReceiveBeginPlay`)

(event `self.ReceiveTick`
  (params (DeltaSeconds :type "Float (single-precision)"))
  (`self.Update Light`)
  (`self.Simple Shadow`)
  (`self.Bake Shadowmap`)
  (`self.RotateLight` DeltaSeconds))

(event `Simple Shadow`
  (bind _returnvalue (`GameplayStatics.GetPlayerPawn` 0))
  (bind _simple_shadow_transition_speed (`self.Simple Shadow Transition Speed`))
  (bind _shadow_check_length_debug (`self.Shadow Check Length Debug`))
  (bind _directional_light_moon (`self.Directional Light Moon`))
  (bind _returnvalue_2 (`self.K2_GetActorLocation` _returnvalue))
  (bind _array (`|MakeArray` _returnvalue :!type "Actor Object Reference"))
  (bind _returnvalue_3 (* (`self.Shadow Check Length`) -1.0))
  (bind _returnvalue_4 (`SceneComponent.GetForwardVector` (`Light.LightComponent` (`self.Directional Light Sun`))))
  ;[1 1 1] Simple Shadow
  (if (`self.Simple Shadows?`)
    (`/Engine/EditorBlueprintResources/StandardMacros.IsValid` (`self.Directional Light Sun`)
      (:`Is Valid`
        (if (`KismetSystemLibrary.IsValid` _directional_light_moon)
          (bind (_outhit _returnvalue_5) (`KismetSystemLibrary.LineTraceSingle` _returnvalue_2 (+ _returnvalue_2 (* (`KismetMathLibrary.VLerp` (`SceneComponent.GetForwardVector` (`Light.LightComponent` _directional_light_moon)) _returnvalue_4 (`KismetMathLibrary.Conv_BoolToDouble` (> (`KismetMathLibrary.NormalizeToRange` (`KismetMathLibrary.Dot_VectorVector` (* _returnvalue_4 -1.0) (`SceneComponent.GetUpVector` (`self.DefaultSceneRoot`))) 0.0 1.0) 0.0))) _returnvalue_3)) "TraceTypeQuery1" false _array _shadow_check_length_debug true (struct :`R` 1.0 :`A` 1.0) (struct :`G` 1.0 :`A` 1.0) 1.0))
          (bind _returnvalue_6 (`KismetMaterialLibrary.GetScalarParameterValue` "/Game/CartoonCelShader/Materials/MaterialCollections/MPC_DirectionalAndSkylight.MPC_DirectionalAndSkylight" "Simple Shadow"))
          (`KismetMaterialLibrary.SetScalarParameterValue` "/Game/CartoonCelShader/Materials/MaterialCollections/MPC_DirectionalAndSkylight.MPC_DirectionalAndSkylight" "Simple Shadow" (`KismetMathLibrary.FInterpTo` _returnvalue_6 (- 1.0 (`KismetMathLibrary.Conv_BoolToDouble` _returnvalue_5)) (`GameplayStatics.GetWorldDeltaSeconds`) _simple_shadow_transition_speed))
          (else
            (bind (_outhit_2 _returnvalue_7) (`KismetSystemLibrary.LineTraceSingle` _returnvalue_2 (+ _returnvalue_2 (* _returnvalue_4 _returnvalue_3)) "TraceTypeQuery1" false _array _shadow_check_length_debug true (struct :`R` 1.0 :`A` 1.0) (struct :`G` 1.0 :`A` 1.0) 1.0))
            (bind _returnvalue_8 (`KismetMaterialLibrary.GetScalarParameterValue` "/Game/CartoonCelShader/Materials/MaterialCollections/MPC_DirectionalAndSkylight.MPC_DirectionalAndSkylight" "Simple Shadow"))
            (`KismetMaterialLibrary.SetScalarParameterValue` "/Game/CartoonCelShader/Materials/MaterialCollections/MPC_DirectionalAndSkylight.MPC_DirectionalAndSkylight" "Simple Shadow" (`KismetMathLibrary.FInterpTo` _returnvalue_8 (- 1.0 (`KismetMathLibrary.Conv_BoolToDouble` _returnvalue_7)) (`GameplayStatics.GetWorldDeltaSeconds`) _simple_shadow_transition_speed)))))
      (:`Is Not Valid`
        (`KismetSystemLibrary.PrintString` "Set the directional light sun parameter! " true true (struct :`G` 0.66 :`B` 1.0 :`A` 1.0) 1.0)))
    (else
      (`KismetMaterialLibrary.SetScalarParameterValue` "/Game/CartoonCelShader/Materials/MaterialCollections/MPC_DirectionalAndSkylight.MPC_DirectionalAndSkylight" "Simple Shadow" 1.0))))

(fn `RotateLight`
  (params (Delta :type "Float (double-precision)"))
  (bind _directional_light_sun (`self.Directional Light Sun`))
  (`/Engine/EditorBlueprintResources/StandardMacros.IsValid` _directional_light_sun
    (:`Is Valid`
      (if (`self.Rotate Sunlight?`)
        (`SceneComponent.K2_AddWorldRotation` (`Light.LightComponent` _directional_light_sun) (`KismetMathLibrary.MakeRotator` 0.0 0.0 (* Delta (`self.Sunlight Rotation Speed`))) false false)))))

(fn `UserConstructionScript`
  (if (`self.Refresh Light Values in Editor`)
    _
    (else
      _))
  (set `self.Refresh Light Values in Editor` false)
  (`KismetMaterialLibrary.SetScalarParameterValue` "/Game/CartoonCelShader/Materials/MaterialCollections/MPC_DirectionalAndSkylight.MPC_DirectionalAndSkylight" "Simple Shadow" 1.0)
  (`self.Update Light`)
  (`self.Bake Shadowmap`)
  (`self.RotateLight` 0.0))