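; BP_ItemDrop is an interactable item-drop actor that shows its interaction menu state through a widget component.
; OnView stores whether the item is actively viewed and passes that state to its WBP_InteractionMenu, which BeginPlay initializes as not in view.
; While the item is viewed, Tick rotates the widget to face the player camera.
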(event `self.ReceiveTick`
  (params (DeltaSeconds :type "Float (single-precision)"))
  (bind _widget (`self.Widget`))
  (if (`self.ActivelyViewed`)
    (`SceneComponent.K2_SetWorldRotation` _widget (`KismetMathLibrary.FindLookAtRotation` (`SceneComponent.K2_GetComponentLocation` _widget) (`SceneComponent.K2_GetComponentLocation` (`PlayerCameraManager.TransformComponent` (`GameplayStatics.GetPlayerCameraManager` 0)))) false false)))

(event `InteractableInterface.OnView`
  (params (InView :type Boolean))
  (bind _output_get (set `self.ActivelyViewed` InView))
  (bind _aswbp_interaction_menu (cast `/Game/MyContent/Blueprints/UI/CombatUI/WBP_InteractionMenu` (`WidgetComponent.GetWidget` (`self.Widget`))))
  (`/Game/MyContent/Blueprints/UI/CombatUI/WBP_InteractionMenu.InView` _aswbp_interaction_menu _output_get))

(event `self.ReceiveBeginPlay`
  (bind _aswbp_interaction_menu (cast `/Game/MyContent/Blueprints/UI/CombatUI/WBP_InteractionMenu` (`WidgetComponent.GetWidget` (`self.Widget`))))
  (`/Game/MyContent/Blueprints/UI/CombatUI/WBP_InteractionMenu.InView` _aswbp_interaction_menu false))

(fn `UserConstructionScript`)