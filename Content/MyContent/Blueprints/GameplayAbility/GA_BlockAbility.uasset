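; Gameplay ability for a guard block that plays a montage and grants damage reduction while held.
; Activation starts GuardMontage at StartBlock, applies GE_Block through a 0.3-second timer, and listens via WaitCancel.
; Cancel removes Block-tagged effects, stops the montage and ends the ability, without clearing the timer.
; OnEndAbility removes effects granting the NormalAttack input tag; debug prints mark each stage.
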(event `self.K2_OnEndAbility`
  (params (bWasCancelled :type Boolean))
  (`self.BP_RemoveGameplayEffectFromOwnerWithGrantedTags` (struct :`GameplayTags` (struct :`(TagName` "Ability.Input.NormalAttack") :`(TagName` "Ability.Input.Skill")))))

(event `GrantDMGReduction`
  (`self.BP_ApplyGameplayEffectToOwner` "/Game/MyContent/Blueprints/GameplayEffect/GE_Block.GE_Block_C")
  (`KismetSystemLibrary.PrintString` "Block Active"))

(event `self.K2_ActivateAbility`
  (`AbilityTask_PlayMontageAndWait.CreatePlayMontageAndWaitProxy` "None" (`self.GuardMontage`) 1.0 "StartBlock"
    (:`then`
      (`KismetSystemLibrary.K2_SetTimerDelegate` (delegate `GrantDMGReduction`) 0.3)
      (`AbilityTask_WaitCancel.WaitCancel`
        (:`then`
          (`KismetSystemLibrary.PrintString` "Start Block"))
        (:`OnCancel`
          (`self.BP_RemoveGameplayEffectFromOwnerWithGrantedTags` (struct :`GameplayTags` (struct :`(TagName` "Effect.Defensive.Block"))))
          (bind _ascharacter (cast `Character` (`self.GetAvatarActorFromActorInfo`)))
          (`Character.StopAnimMontage` _ascharacter null)
          (`self.K2_EndAbility`)
          (`KismetSystemLibrary.PrintString` "Release Block"))))))