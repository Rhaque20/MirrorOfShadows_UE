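; Player gameplay ability for a normal melee attack, playing the montage for the current chain step.
; Activation applies the in-attack effect, flags the character as attacking, disables movement and picks attack data by chain index.
; An attack gameplay event triggers a scaled hit-zone scan, hit processing and a sequence counter increment.
; A recover event or montage cancellation removes effects granting the normal-attack input tag; montage exits end the ability.
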(event `self.K2_ActivateAbility`
  (`self.K2_CommitAbility`)
  (bind _asbp_player (cast `/Game/MyContent/Blueprints/Character_BP/BP_Player` (`self.GetAvatarActorFromActorInfo`))
    (:`then`
      (`/Engine/EditorBlueprintResources/StandardMacros.IsValid` _asbp_player
        (:`Is Valid`
          (bind _output_get (set `self.AbilityOwner` _asbp_player))
          (`self.BP_ApplyGameplayEffectToOwner` "/Game/MyContent/Blueprints/GameplayEffect/GE_InAttack.GE_InAttack_C")
          (bind _charactercore (`PlayerCharacters.CharacterCore` _output_get))
          (set `CombatComponent.bIsAttacking` true _charactercore)
          (set `PlayerCharacters.CanMove` false _output_get)
          (bind _output (`|GetArrayItem` (`self.NormalAttacks`) (`PlayerCore.CurrentChain` _charactercore)))
          (set `self.AttackData` _output)
          (`AbilityTask_PlayMontageAndWait.CreatePlayMontageAndWaitProxy` "None" (`Skill.GetAnimation` _output 0) 1.0 "None" true 1.0 0.0 true
            (:`then`
              (`|ExecutionSequence`
                (:`then_0`
                  (`AbilityTask_WaitGameplayEvent.WaitGameplayEvent` (struct :`TagName` "Event.Melee.Attack") null
                    (:`EventReceived`
                      (bind _outhits (`self.HitZoneScan` (`Skill.GetHitBoxScale` (`self.AttackData`))))
                      (`self.ProcessHits` _outhits)
                      (bind _result (`/Engine/EditorBlueprintResources/StandardMacros.IncrementInt` (`self.HitSequence_0`))
                        (:`  `
                          (set `self.HitSequence_0` _result))))))
                (:`then_1`
                  (`AbilityAsync_WaitGameplayEvent.WaitGameplayEventToActor` (`self.GetAvatarActorFromActorInfo`) (struct :`TagName` "Event.Melee.Recover")
                    (:`EventReceived`
                      (`self.BP_RemoveGameplayEffectFromOwnerWithGrantedTags` (struct :`GameplayTags` (struct :`(TagName` "Ability.Input.NormalAttack")))))))))
            (:`OnCompleted`
              (`self.K2_EndAbility` :!label _label))
            (:`OnBlendOut`
              (goto _label))
            (:`OnInterrupted`
              (goto _label))
            (:`OnCancelled`
              (`KismetSystemLibrary.PrintString` "Montage Canceled")
              (`self.BP_RemoveGameplayEffectFromOwnerWithGrantedTags` (struct :`GameplayTags` (struct :`(TagName` "Ability.Input.NormalAttack"))))
              (goto _label))))
        (:`Is Not Valid`
          (`self.K2_EndAbility` :!label _label_2))))
    (:`CastFailed`
      (goto _label_2))))