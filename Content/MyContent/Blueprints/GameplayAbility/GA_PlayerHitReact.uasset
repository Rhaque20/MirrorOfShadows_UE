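; Gameplay ability that handles the player's hit reaction, built on a parent ability's activation logic.
; On activation it prints a debug string, then casts the avatar to BP_Player and gets its BP_StaggerComponent.
; It copies that component's StaggerAnimTest into RegularStagger before calling the parent ActivateAbility, which runs only if those casts and the validity check succeed.
; The OnEndAbility override is disabled.
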(event `self.K2_ActivateAbility`
  (`KismetSystemLibrary.PrintString` "PlayerHitReactStart")
  (bind _asbp_player (cast `/Game/MyContent/Blueprints/Character_BP/BP_Player` (`self.GetAvatarActorFromActorInfo`)))
  (`/Engine/EditorBlueprintResources/StandardMacros.IsValid` _asbp_player
    (:`Is Valid`
      (bind _asbp_stagger_component (cast `/Game/MyContent/Blueprints/Cores/BP_StaggerComponent` (`PlayerCharacters.StaggerComponent` _asbp_player)))
      (set `self.RegularStagger` (`/Game/MyContent/Blueprints/Cores/BP_StaggerComponent.StaggerAnimTest` _asbp_stagger_component))
      (`parent.K2_ActivateAbility`))))