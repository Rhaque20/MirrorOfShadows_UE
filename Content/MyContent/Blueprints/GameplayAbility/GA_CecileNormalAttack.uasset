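; Gameplay ability for Cecile's normal melee attack, playing an attack montage and applying a damage effect.
; On commit, it sphere-traces a short distance ahead for pawns, applies GE_Damage to the hit actor and ends, cancelling if commit fails.
; That hit logic runs immediately after starting the Event.Melee.Attack wait, and is also wired from the event through an instant WaitTargetData task.
; Montage completion, interruption or cancellation also ends the ability.
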(event `self.K2_ActivateAbility`
  (bind _returnvalue (`self.GetAvatarActorFromActorInfo`))
  (bind _returnvalue_2 (`Actor.K2_GetActorLocation` _returnvalue))
  (`AbilityTask_PlayMontageAndWait.CreatePlayMontageAndWaitProxy` "None" "/Game/MyContent/Animations/Player/Cecile/CecileMontages/Cecile_NA1_Montage.Cecile_NA1_Montage"
    (:`then`
      (`AbilityTask_WaitGameplayEvent.WaitGameplayEvent` (struct :`TagName` "Event.Melee.Attack") null
        (:`then`
          _)
        (:`EventReceived`
          (`AbilityTask_WaitTargetData.WaitTargetData` "None" "Instant"
            (:`then`
              _))))
      (bind _returnvalue_3 (`self.K2_CommitAbility`))
      (if _returnvalue_3
        (bind _outhit (`KismetSystemLibrary.SphereTraceSingleForObjects` _returnvalue_2 (+ _returnvalue_2 (* (`Actor.GetActorForwardVector` _returnvalue) 100.0)) 50.0 (`|MakeArray` "ObjectTypeQuery3" :!type "EObjectTypeQuery Enum") false (`|MakeArray` _returnvalue) "Persistent"))
        (`self.BP_ApplyGameplayEffectToTarget` (`AbilitySystemBlueprintLibrary.AbilityTargetDataFromActor` (`.HitActor` (`GameplayStatics.BreakHitResult` _outhit))) "/Game/MyContent/Blueprints/GameplayEffect/GE_Damage.GE_Damage_C")
        (`self.K2_EndAbility`)
        (`KismetSystemLibrary.PrintString` "Comitted")
        (else
          (`self.K2_CancelAbility`)
          (`KismetSystemLibrary.PrintString` "Couldn't commit"))))
    (:`OnCompleted`
      (`self.K2_EndAbility` :!label _label))
    (:`OnInterrupted`
      (goto _label))
    (:`OnCancelled`
      (goto _label))))