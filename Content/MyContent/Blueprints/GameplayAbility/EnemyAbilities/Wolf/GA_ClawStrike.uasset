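; GA_ClawStrike is the wolf enemy's claw strike gameplay ability.
; Activation defers entirely to the parent ability class, so the strike behavior itself lives there.
; When the ability ends, cancelled or not, it casts AttackData to EnemySkill and applies a GE_Cooldown spec to the owner, with duration set from that skill's MaxCooldown.
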(event `self.K2_ActivateAbility`
  (`parent.K2_ActivateAbility`))

(event `self.K2_OnEndAbility`
  (params (bWasCancelled :type Boolean))
  (`parent.K2_OnEndAbility` bWasCancelled)
  (bind _asenemy_skill (cast `EnemySkill` (`self.AttackData`)))
  (bind _returnvalue (`AbilitySystemBlueprintLibrary.SetDuration` (`AbilitySystemComponent.MakeOutgoingSpec` :`self` (`RPGCharacterBase.AbilitySystem` (`self.AbilityOwner`)) :`GameplayEffectClass` "/Game/MyContent/Blueprints/GameplayEffect/Cooldowns/Enemy/GE_Cooldown.GE_Cooldown_C") (`EnemySkill.MaxCooldown` _asenemy_skill)))
  (`self.K2_ApplyGameplayEffectSpecToOwner` _returnvalue))