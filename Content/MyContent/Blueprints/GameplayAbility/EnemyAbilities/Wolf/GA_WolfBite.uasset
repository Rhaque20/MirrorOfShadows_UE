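; Wolf bite melee Gameplay Ability that plays the active enemy skill's montage with motion hyper armor and an in-attack effect.
; Montage gameplay events trigger a box-trace hit scan or recovery.
; Hits apply damage, poise damage, camera shake and hit stop, then branch into perfect-dodge slowdown, parry stance damage on the wolf, or player stagger.
; Ending applies a delay effect lasting the skill's internal cooldown.
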(event `self.K2_OnEndAbility`
  (params (bWasCancelled :type Boolean))
  (bind _returnvalue (`AbilitySystemBlueprintLibrary.GetAbilitySystemComponent` (`self.GetAvatarActorFromActorInfo`)))
  (`self.ApplyMotionHyperArmor` false)
  (if (`self.WasInterrupted`)
    (`self.BP_RemoveGameplayEffectFromOwnerWithGrantedTags` (struct :`GameplayTags` (struct :`(TagName` "Ability.Input.NormalAttack")))))
  (bind _asenemy_skill (cast `EnemySkill` (`self.AttackData`)))
  (bind _returnvalue_2 (`AbilitySystemBlueprintLibrary.SetDuration` (`AbilitySystemComponent.MakeOutgoingSpec` :`self` _returnvalue :`GameplayEffectClass` "/Game/MyContent/GE_AttackDelay.GE_AttackDelay_C") (`EnemySkill.InternalCooldown` _asenemy_skill)))
  (`AbilitySystemComponent.BP_ApplyGameplayEffectSpecToSelf` _returnvalue _returnvalue_2)
  (`KismetSystemLibrary.PrintString` "Internal Cooldown Activated"))

(event `self.K2_ActivateAbility`
  (bind _returnvalue (`self.GetAvatarActorFromActorInfo`))
  (bind _attackdata (`self.AttackData`))
  (`self.K2_CommitAbility`)
  (`self.ApplyMotionHyperArmor` true)
  (bind _asbp_enemy_base (cast `/Game/MyContent/Blueprints/Enemy_BP/BP_EnemyBase` _returnvalue)
    (:`then`
      (`/Engine/EditorBlueprintResources/StandardMacros.IsValid` _asbp_enemy_base
        (:`Is Valid`
          (bind _output_get (set `self.AbilityOwner` _asbp_enemy_base))
          (set `self.AttackData` (`/Game/MyContent/Blueprints/Enemy_BP/BP_EnemyBase.ActiveSkill` _asbp_enemy_base))
          (`AbilitySystemComponent.BP_ApplyGameplayEffectToSelf` :`self` (`AbilitySystemBlueprintLibrary.GetAbilitySystemComponent` _returnvalue) :`GameplayEffectClass` "/Game/MyContent/Blueprints/GameplayEffect/GE_InAttack.GE_InAttack_C")
          (`self.BP_ApplyGameplayEffectToOwner` "/Game/MyContent/Blueprints/GameplayEffect/GE_InAttack.GE_InAttack_C")
          (set `EnemyCharacterBase.IsAttacking` true _output_get)
          (`AbilityTask_PlayMontageAndWait.CreatePlayMontageAndWaitProxy` "None" (`Skill.GetAnimation` _attackdata 0)
            (:`then`
              (`|ExecutionSequence`
                (:`then_0`
                  (`AbilityTask_WaitGameplayEvent.WaitGameplayEvent` (struct :`TagName` "Event.Melee.Attack") null
                    (:`EventReceived`
                      (bind _outhits (`self.HitZoneScan` (`Skill.HitBoxScale` _attackdata)))
                      (`self.ProcessHits` _outhits))))
                (:`then_1`
                  (`AbilityAsync_WaitGameplayEvent.WaitGameplayEventToActor` (`self.AbilityOwner`) (struct :`TagName` "Event.Melee.Recover")
                    (:`EventReceived`
                      (`self.BP_RemoveGameplayEffectFromOwnerWithGrantedTags` (struct :`GameplayTags` (struct :`(TagName` "Ability.Input.NormalAttack"))))
                      (`EnemyCharacterBase.Recover` (`self.AbilityOwner`)))))))
            (:`OnCompleted`
              (`self.K2_EndAbility` :!label _label))
            (:`OnBlendOut`
              (goto _label))
            (:`OnInterrupted`
              (goto _label))
            (:`OnCancelled`
              (goto _label))))
        (:`Is Not Valid`
          (`self.K2_EndAbility` :!label _label_2))))
    (:`CastFailed`
      (goto _label_2))))

(fn `ActivateOnHit`
  (params (HitTarget :type "Pawn Object Reference"))
  (bind _asbp_player (cast `/Game/MyContent/Blueprints/Character_BP/BP_Player` HitTarget))
  (bind _asbp_player_stagger (cast `/Game/MyContent/Blueprints/Cores/BP_PlayerStagger` (`PlayerCharacters.StaggerComponent` _asbp_player)))
  (`/Game/MyContent/Blueprints/Cores/BP_StaggerComponent.OnHit` _asbp_player_stagger))

(fn `HitResponse`
  (params (HitTarget :type "Pawn Object Reference"))
  (bind _returnvalue (`AbilitySystemBlueprintLibrary.GetAbilitySystemComponent` HitTarget))
  (if (`GameplayTagAssetInterface.HasMatchingGameplayTag` _returnvalue (struct :`TagName` "Effect.Defensive.PerfectDodge"))
    (`KismetSystemLibrary.PrintString` "Perfect Dodge")
    (bind _asbp_player_state (cast `/Game/MyContent/Blueprints/Miscellaneous/BP_PlayerState` (`GameplayStatics.GetPlayerState` 0)))
    (`/Engine/EditorBlueprintResources/StandardMacros.IsValid` _asbp_player_state
      (:`Is Valid`
        (`/Game/MyContent/Blueprints/Miscellaneous/BP_PlayerState.TriggerEvadeSlowDown` _asbp_player_state (`self.AbilityOwner`))))
    (elif (`GameplayTagAssetInterface.HasMatchingGameplayTag` _returnvalue (struct :`TagName` "Effect.Defensive.Parry"))
      (`KismetSystemLibrary.PrintString` "PARRY!")
      (`self.BP_ApplyGameplayEffectToOwner` "/Game/MyContent/Blueprints/GameplayEffect/GE_StanceDamage.GE_StanceDamage_C")
      (else
        (`self.ActivateOnHit` null)))))

(fn `HitZoneScan`
  (params (HitBoxScale :type "Vector Structure"))
  (returns (OutHits :type "Array of HitResult Structure"))
  (bind _returnvalue (`self.GetAvatarActorFromActorInfo`))
  (bind (_hurtboxspot _finalhurtboxspot) (`/Game/MyContent/Blueprints/Enemy_BP/BP_EnemyBase.SetHurtboxSpot` (`self.AbilityOwner`) (`Skill.HitBoxLocation` (`self.AttackData`))))
  (bind _outhits (`KismetSystemLibrary.BoxTraceMulti` _hurtboxspot _finalhurtboxspot (* HitBoxScale (32.0 32.0 32.0)) (`Actor.K2_GetActorRotation` _returnvalue) "TraceTypeQuery3" false (`|MakeArray` _returnvalue) "ForDuration"))
  (if (== (`KismetArrayLibrary.Array_Length` _outhits) 0)
    (`KismetSystemLibrary.PrintString` "Hit nothing"))
  (return _outhits))

(fn `ProcessHits`
  (params (Array :type "Array of HitResult Structure (by ref)"))
  (locals (TriggeredShake :type Boolean :default false) (HitActors :type "Array of Actor Object Reference"))
  (bind _attackdata (`self.AttackData`))
  (bind _hitactors (`local.HitActors`))
  (bind _abilityowner (`self.AbilityOwner`))
  (if (> (`KismetArrayLibrary.Array_Length` Array) 0)
    (if (`Skill.HasDifferentMods` _attackdata)
      (`EnemyCharacterBase.SetSkillModifier` _abilityowner (`Skill.ReturnModfierAtSequence` _attackdata (`self.HitSequence`)))
      (else
        (`EnemyCharacterBase.SetSkillModifier` _abilityowner (`Skill.ReturnModifier` _attackdata))))
    (for _array_element Array
      (bind (_bblockinghit _binitialoverlap _time _distance _location _impactpoint _normal _impactnormal _physmat _hitactor) (`GameplayStatics.BreakHitResult` _array_element))
      (if (`KismetArrayLibrary.Array_Contains` (`Actor.Tags` _hitactor) (`self.TargetTag`))
        (bind _returnvalue (`Actor.GetOwner` _hitactor))
        (if (not (`KismetArrayLibrary.Array_Contains` _hitactors _returnvalue))
          (if (not (`local.TriggeredShake`))
            (`GameplayStatics.PlayWorldCameraShake` "/Game/MyContent/Blueprints/Miscellaneous/BP_MatineeCameraShake.BP_MatineeCameraShake_C" (`Actor.K2_GetActorLocation` (`self.GetAvatarActorFromActorInfo`)) 0.0 500.0)
            (`/Game/MyContent/Blueprints/Enemy_BP/BP_EnemyBase.StartHitStop` (`self.AbilityOwner`))
            (set `local.TriggeredShake` true))
          (`KismetArrayLibrary.Array_Add` _hitactors _returnvalue)
          (bind _returnvalue_2 (`AbilitySystemBlueprintLibrary.AbilityTargetDataFromActor` _hitactor))
          (`self.BP_ApplyGameplayEffectToTarget` _returnvalue_2 "/Game/MyContent/Blueprints/GameplayEffect/GE_Damage.GE_Damage_C")
          (`self.ApplyPoiseDamage` _returnvalue_2 _returnvalue)
          (bind _asbp_character_controller (cast `/Game/MyContent/Blueprints/Character_BP/BP_CharacterController` _returnvalue))
          (`/Engine/EditorBlueprintResources/StandardMacros.IsValid` _asbp_character_controller
            (:`Is Valid`
              (`self.HitResponse` (`Controller.K2_GetPawn` _asbp_character_controller)))))))
    (return)))