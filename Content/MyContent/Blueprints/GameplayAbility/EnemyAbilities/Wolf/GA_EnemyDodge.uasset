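; GA_EnemyDodge is a gameplay ability that makes an enemy, filed under Wolf, play a dodge montage with an evade effect.
; On activation it commits, clears effects granting the evade cooldown tag, and applies GE_Evade to itself through a SetByCaller magnitude.
; Any montage outcome ends the ability, and ending applies GE_EvadeCD, so the cooldown effect is applied after the dodge.
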(event `self.K2_OnEndAbility`
  (params (bWasCancelled :type Boolean))
  (`AbilitySystemComponent.BP_ApplyGameplayEffectToSelf` :`self` (`AbilitySystemBlueprintLibrary.GetAbilitySystemComponent` (`self.GetAvatarActorFromActorInfo`)) :`GameplayEffectClass` "/Game/MyContent/Blueprints/GameplayEffect/Cooldowns/Enemy/GE_EvadeCD.GE_EvadeCD_C"))

(event `self.K2_ActivateAbility`
  (bind _returnvalue (`AbilitySystemBlueprintLibrary.GetAbilitySystemComponent` (`self.GetAvatarActorFromActorInfo`)))
  (`self.K2_CommitAbility`)
  (`AbilitySystemComponent.RemoveActiveEffectsWithAppliedTags` _returnvalue (struct :`GameplayTags` (struct :`(TagName` "Skill.Cooldown.Evade"))))
  (bind _returnvalue_2 (`AbilitySystemBlueprintLibrary.AssignTagSetByCallerMagnitude` (`AbilitySystemComponent.MakeOutgoingSpec` :`self` _returnvalue :`GameplayEffectClass` "/Game/MyContent/Blueprints/GameplayEffect/GE_Evade.GE_Evade_C") (struct :`TagName` "Effect.Defensive.Evade") 0.5))
  (`AbilitySystemComponent.BP_ApplyGameplayEffectSpecToSelf` _returnvalue _returnvalue_2)
  (`AbilityTask_PlayMontageAndWait.CreatePlayMontageAndWaitProxy` "None" (`self.DodgeMontage`)
    (:`OnCompleted`
      _)
    (:`OnBlendOut`
      _)
    (:`OnInterrupted`
      _)
    (:`OnCancelled`
      _))
  (`self.K2_EndAbility`))