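; Gameplay ability for a player character's normal melee attack, playing the montage for the current combo chain step.
; Activation applies GE_InAttack, flags the character as attacking and disables its movement.
; A melee Attack event triggers a forward box trace scaled per attack, applying GE_Damage while tracking owners already hit.
; A Recover event removes effects granting the NormalAttack input tag and ends the ability.
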(event `self.K2_ActivateAbility`
  (`self.K2_CommitAbility`)
  (`KismetSystemLibrary.PrintString` "Activating Ability")
  (bind _asplayer_characters (cast `PlayerCharacters` (`self.GetAvatarActorFromActorInfo`))
    (:`then`
      (`self.BP_ApplyGameplayEffectToOwner` "/Game/MyContent/Blueprints/GameplayEffect/GE_InAttack.GE_InAttack_C")
      (bind _charactercore (`PlayerCharacters.CharacterCore` _asplayer_characters))
      (set `CombatComponent.bIsAttacking` true _charactercore)
      (set `PlayerCharacters.CanMove` false _asplayer_characters)
      (bind _output (`|GetArrayItem` (`self.NormalAttacks`) (`PlayerCore.CurrentChain` _charactercore)))
      (`AbilityTask_PlayMontageAndWait.CreatePlayMontageAndWaitProxy` "None" (`Skill.GetAnimation` _output 0) 1.0 "None" true 1.0 0.0 true
        (:`then`
          (`|ExecutionSequence`
            (:`then_0`
              (`AbilityTask_WaitGameplayEvent.WaitGameplayEvent` (struct :`TagName` "Event.Melee.Attack") null
                (:`EventReceived`
                  (bind _outhits (`self.HitZoneScan` (`Skill.HitBoxScale` _output)))
                  (`self.ProcessHits` _outhits))))
            (:`then_1`
              (`AbilityAsync_WaitGameplayEvent.WaitGameplayEventToActor` (`self.GetAvatarActorFromActorInfo`) (struct :`TagName` "Event.Melee.Recover")
                (:`EventReceived`
                  (`self.BP_RemoveGameplayEffectFromOwnerWithGrantedTags` (struct :`GameplayTags` (struct :`(TagName` "Ability.Input.NormalAttack"))))
                  (`self.K2_EndAbility`))))))))
    (:`CastFailed`
      (`self.K2_EndAbility`))))

(fn `HitZoneScan`
  (params (HitBoxScale :type "Vector Structure"))
  (returns (OutHits :type "Array of HitResult Structure"))
  (bind _returnvalue (`self.GetAvatarActorFromActorInfo`))
  (bind _returnvalue_2 (+ (`Actor.K2_GetActorLocation` _returnvalue) (* 100.0 (`Actor.GetActorForwardVector` _returnvalue))))
  (bind _outhits (`KismetSystemLibrary.BoxTraceMulti` _returnvalue_2 (+ _returnvalue_2 (0.1 0.1 0.1)) (* HitBoxScale (32.0 32.0 32.0)) (`Actor.K2_GetActorRotation` _returnvalue) "TraceTypeQuery3" false (`|MakeArray` _returnvalue) "ForDuration"))
  (return _outhits))

(fn `ProcessHits`
  (params (Array :type "Array of HitResult Structure (by ref)"))
  (bind _array (`|MakeArray` null :!type "Actor Object Reference"))
  (for (_array_element _array_index) Array
    (bind (_bblockinghit _binitialoverlap _time _distance _location _impactpoint _normal _impactnormal _physmat _hitactor) (`GameplayStatics.BreakHitResult` _array_element))
    (bind _returnvalue (`Actor.GetOwner` _hitactor))
    (if (`KismetArrayLibrary.Array_Contains` _array _returnvalue)
      (`KismetSystemLibrary.PrintString` "Already hit this target")
      (else
        (`KismetArrayLibrary.Array_Add` _array _returnvalue)
        (`KismetSystemLibrary.PrintString` (`KismetStringLibrary.Conv_IntToString` _array_index))
        (`self.BP_ApplyGameplayEffectToTarget` (`AbilitySystemBlueprintLibrary.AbilityTargetDataFromActor` _hitactor) "/Game/MyContent/Blueprints/GameplayEffect/GE_Damage.GE_Damage_C")))))