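; Generic player skill Gameplay Ability that plays the active skill's montage, applies attack and skill effects, and locks movement.
; Each melee attack event runs a forward box trace scaled by skill data, then advances the hit sequence.
; Hits apply GE_Damage once per target owner, using per-sequence or shared skill modifiers, with one camera shake and hit-stop.
; A recover event removes effects granting the normal-attack input tag.
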(event `self.K2_ActivateAbility`
  (`self.K2_CommitAbility`)
  (bind _asbp_player (cast `/Game/MyContent/Blueprints/Character_BP/BP_Player` (`self.GetAvatarActorFromActorInfo`))
    (:`then`
      (bind _output_get (set `self.AbilityOwner` _asbp_player))
      (`self.BP_ApplyGameplayEffectToOwner` "/Game/MyContent/Blueprints/GameplayEffect/GE_InAttack.GE_InAttack_C")
      (`self.BP_ApplyGameplayEffectToOwner` "/Game/MyContent/Blueprints/GameplayEffect/GE_InSkill.GE_InSkill_C")
      (set `CombatComponent.bIsAttacking` true (`PlayerCharacters.CharacterCore` _output_get))
      (set `PlayerCharacters.CanMove` false _output_get)
      (bind _output_get_2 (set `self.AttackData` (`/Game/MyContent/Blueprints/Character_BP/BP_Player.ActiveSkill` _asbp_player)))
      (`AbilityTask_PlayMontageAndWait.CreatePlayMontageAndWaitProxy` "None" (`Skill.GetAnimation` _output_get_2 0) 1.0 "None" true 1.0 0.0 true
        (:`then`
          (`|ExecutionSequence`
            (:`then_0`
              (`AbilityTask_WaitGameplayEvent.WaitGameplayEvent` (struct :`TagName` "Event.Melee.Attack") null
                (:`EventReceived`
                  (bind _outhits (`self.HitZoneScan` (`Skill.HitBoxScale` _output_get_2)))
                  (`self.ProcessHits` _outhits)
                  (bind _result (`/Engine/EditorBlueprintResources/StandardMacros.IncrementInt` (`self.HitSequence`))
                    (:`  `
                      (set `self.HitSequence` _result))))))
            (:`then_1`
              (`AbilityAsync_WaitGameplayEvent.WaitGameplayEventToActor` (`self.GetAvatarActorFromActorInfo`) (struct :`TagName` "Event.Melee.Recover")
                (:`EventReceived`
                  (`self.BP_RemoveGameplayEffectFromOwnerWithGrantedTags` (struct :`GameplayTags` (struct :`(TagName` "Ability.Input.NormalAttack")))))))))
        (:`OnCompleted`
          (`self.K2_EndAbility` :!label _label))
        (:`OnBlendOut`
          (goto _label))
        (:`OnInterrupted`
          (goto _label))
        (:`OnCancelled`
          (goto _label))))
    (:`CastFailed`
      (`self.K2_EndAbility`))))

(fn `HitZoneScan`
  (params (HitBoxScale :type "Vector Structure"))
  (returns (OutHits :type "Array of HitResult Structure"))
  (bind _returnvalue (`self.GetAvatarActorFromActorInfo`))
  (bind _returnvalue_2 (+ (`Actor.K2_GetActorLocation` _returnvalue) (* 100.0 (`Actor.GetActorForwardVector` _returnvalue))))
  (bind _outhits (`KismetSystemLibrary.BoxTraceMulti` _returnvalue_2 (+ _returnvalue_2 (0.1 0.1 0.1)) (* HitBoxScale (32.0 32.0 32.0)) (`Actor.K2_GetActorRotation` _returnvalue) "TraceTypeQuery4" false (`|MakeArray` _returnvalue) "ForDuration"))
  (if (== (`KismetArrayLibrary.Array_Length` _outhits) 0)
    (`KismetSystemLibrary.PrintString` "Hit nothing"))
  (return _outhits))

(fn `ProcessHits`
  (params (Array :type "Array of HitResult Structure (by ref)"))
  (locals (TriggeredShake :type Boolean))
  (bind _array (`|MakeArray` null :!type "Actor Object Reference"))
  (bind _attackdata (`self.AttackData`))
  (if (> (`KismetArrayLibrary.Array_Length` Array) 0)
    (bind _asbp_player (cast `/Game/MyContent/Blueprints/Character_BP/BP_Player` (`self.GetAvatarActorFromActorInfo`)))
    (if (`Skill.HasDifferentMods` _attackdata)
      (`PlayerCharacters.SetSkillModifier` _asbp_player (`Skill.ReturnModfierAtSequence` _attackdata (`self.HitSequence`)))
      (else
        (`PlayerCharacters.SetSkillModifier` _asbp_player (`Skill.ReturnModifier` _attackdata))))
    (for _array_element Array
      (bind (_bblockinghit _binitialoverlap _time _distance _location _impactpoint _normal _impactnormal _physmat _hitactor) (`GameplayStatics.BreakHitResult` _array_element))
      (bind _returnvalue (`Actor.GetOwner` _hitactor))
      (if (`KismetArrayLibrary.Array_Contains` _array _returnvalue)
        (`KismetSystemLibrary.PrintString` "Already hit this target")
        (else
          (if (not (`local.TriggeredShake`))
            (`GameplayStatics.PlayWorldCameraShake` "/Game/MyContent/Blueprints/Miscellaneous/BP_MatineeCameraShake.BP_MatineeCameraShake_C" (`Actor.K2_GetActorLocation` (`self.GetAvatarActorFromActorInfo`)) 0.0 500.0)
            (`/Game/MyContent/InterfaceBlueprints/BPI_HitStop.StartHitStop` (`self.AbilityOwner`))
            (set `local.TriggeredShake` true))
          (`KismetArrayLibrary.Array_Add` _array _returnvalue)
          (`self.BP_ApplyGameplayEffectToTarget` (`AbilitySystemBlueprintLibrary.AbilityTargetDataFromActor` _hitactor) "/Game/MyContent/Blueprints/GameplayEffect/GE_Damage.GE_Damage_C"))))))