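; Gameplay ability for player melee attacks, providing hit, damage and interrupt helpers around an empty ActivateAbility.
; HitZoneScan box-traces ahead of the avatar; ProcessHits filters by tag, deduplicates victims and triggers camera shake and hit stop once.
; Hits notify the victim's StaggerComponent, then apply physical damage plus AttackData-driven poise damage and poise freeze effects.
; Other helpers toggle interrupt-resisting hyper armor via SetByCaller effects, check interrupt tags and compare facing.
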(event `self.K2_ActivateAbility`)

(fn `ActivateOnHit`
  (params (HitTarget :type "Pawn Object Reference"))
  (bind _asrpgcharacter_base (cast `RPGCharacterBase` HitTarget))
  (`StaggerComponent.OnHit` (`RPGCharacterBase.StaggerComponent` _asrpgcharacter_base)))

(fn `ApplyMotionHyperArmor`
  (params (ApplyMotionArmor :type Boolean))
  (if ApplyMotionArmor
    (bind _returnvalue (`AbilitySystemBlueprintLibrary.AssignTagSetByCallerMagnitude` (`AbilitySystemComponent.MakeOutgoingSpec` :`self` (`AbilitySystemBlueprintLibrary.GetAbilitySystemComponent` (`self.GetAvatarActorFromActorInfo`)) :`GameplayEffectClass` "/Game/MyContent/Blueprints/GameplayEffect/PoiseSystem/GE_MotionArmor.GE_MotionArmor_C") (struct :`TagName` "Stats.Percent.InterruptRes") (`Skill.ResistInterruptMod` (`self.AttackData`))))
    (`self.K2_ApplyGameplayEffectSpecToOwner` _returnvalue)
    (else
      (`self.BP_RemoveGameplayEffectFromOwnerWithGrantedTags` (struct :`GameplayTags` (struct :`(TagName` "Stats.Percent.InterruptRes")))))))

(fn `ApplyPoiseDamage`
  (bind _attacktarget (`self.AttackTarget`))
  (bind _returnvalue (`AbilitySystemBlueprintLibrary.GetAbilitySystemComponent` _attacktarget))
  (bind _returnvalue_2 (`AbilitySystemBlueprintLibrary.AbilityTargetDataFromActor` _attacktarget))
  (bind _returnvalue_3 (`AbilitySystemBlueprintLibrary.AssignTagSetByCallerMagnitude` (`AbilitySystemComponent.MakeOutgoingSpec` :`self` _returnvalue :`GameplayEffectClass` "/Game/MyContent/Blueprints/GameplayEffect/PoiseSystem/GE_PoiseDamage.GE_PoiseDamage_C") (struct :`TagName` "Damage.Stagger.Poise") (* (`Skill.ReturnPoiseDamage` (`self.AttackData`) 0) (`.ReturnValue` (`AbilitySystemBlueprintLibrary.GetFloatAttributeFromAbilitySystemComponent` _returnvalue (struct :`AttributeName` "PoiseMod" :`Attribute` "/Script/MirrorOfShadows.BaseAttributeSet:PoiseMod" :`AttributeOwner` "/Script/CoreUObject.Class'/Script/MirrorOfShadows.BaseAttributeSet'"))))))
  (`self.K2_ApplyGameplayEffectSpecToTarget` _returnvalue_3 _returnvalue_2)
  (`AbilitySystemComponent.RemoveActiveEffectsWithGrantedTags` _returnvalue (struct :`GameplayTags` (struct :`(TagName` "Damage.Stagger.Poise"))))
  (`self.K2_ApplyGameplayEffectSpecToTarget` (`AbilitySystemComponent.MakeOutgoingSpec` :`self` _returnvalue :`GameplayEffectClass` "/Game/MyContent/Blueprints/GameplayEffect/PoiseSystem/GE_PoiseFreeze.GE_PoiseFreeze_C") _returnvalue_2))

(fn `HitResponse`
  (params (HitTarget :type "Pawn Object Reference"))
  (returns (DidHit :type Boolean))
  (`self.ActivateOnHit` HitTarget)
  (return true))

(fn `HitZoneScan`
  (params (HitBoxScale :type "Vector Structure"))
  (returns (OutHits :type "Array of HitResult Structure"))
  (bind _returnvalue (`self.GetAvatarActorFromActorInfo`))
  (bind _returnvalue_2 (+ (`Actor.K2_GetActorLocation` _returnvalue) (* 100.0 (`Actor.GetActorForwardVector` _returnvalue))))
  (bind _outhits (`KismetSystemLibrary.BoxTraceMulti` _returnvalue_2 (+ _returnvalue_2 (0.1 0.1 0.1)) (* HitBoxScale (32.0 32.0 32.0)) (`Actor.K2_GetActorRotation` _returnvalue) "TraceTypeQuery4" false (`|MakeArray` _returnvalue) "ForDuration"))
  (return _outhits))

(fn `Is in Front`
  (params (TargetToHit :type "Actor Object Reference") (Angle :type "Float (double-precision)"))
  (returns (IsFront :type Boolean))
  (return (<= (`KismetMathLibrary.Dot_VectorVector` (`Actor.GetActorForwardVector` TargetToHit) (`Actor.GetActorForwardVector` (`self.GetAvatarActorFromActorInfo`))) Angle)))

(fn `ProcessHits`
  (params (Array :type "Array of HitResult Structure (by ref)"))
  (locals (TriggeredShake :type Boolean) (HitActors :type "Array of Actor Object Reference") (HitTarget :type "Actor Object Reference"))
  (bind _hitactors (`local.HitActors`))
  (if (> (`KismetArrayLibrary.Array_Length` Array) 0)
    (`KismetSystemLibrary.PrintString` (`KismetStringLibrary.Concat_StrStr` "Skill mod " (`KismetStringLibrary.Conv_DoubleToString` (`.ReturnValue` (`AbilitySystemBlueprintLibrary.GetFloatAttributeFromAbilitySystemComponent` (`AbilitySystemBlueprintLibrary.GetAbilitySystemComponent` (`self.GetAvatarActorFromActorInfo`)) (struct :`AttributeName` "SkillModifier" :`Attribute` "/Script/MirrorOfShadows.BaseAttributeSet:SkillModifier" :`AttributeOwner` "/Script/CoreUObject.Class'/Script/MirrorOfShadows.BaseAttributeSet'"))))))
    (bind _asbp_player (cast `/Game/MyContent/Blueprints/Character_BP/BP_Player` (`self.GetAvatarActorFromActorInfo`)))
    (`PlayerCharacters.SetSkillModifier` _asbp_player (`Skill.ReturnSkillModifier` (`self.AttackData`) (`self.HitSequence`)))
    (for _array_element Array
      (bind (_bblockinghit _binitialoverlap _time _distance _location _impactpoint _normal _impactnormal _physmat _hitactor) (`GameplayStatics.BreakHitResult` _array_element))
      (if (`KismetArrayLibrary.Array_Contains` (`Actor.Tags` _hitactor) (`self.TargetTag`))
        (bind _returnvalue (`Actor.GetOwner` _hitactor))
        (if (not (`KismetArrayLibrary.Array_Contains` _hitactors _returnvalue))
          (if (not (`local.TriggeredShake`))
            (`GameplayStatics.PlayWorldCameraShake` "/Game/MyContent/Blueprints/Miscellaneous/BP_MatineeCameraShake.BP_MatineeCameraShake_C" (`Actor.K2_GetActorLocation` (`self.GetAvatarActorFromActorInfo`)) 0.0 500.0)
            (`/Game/MyContent/InterfaceBlueprints/BPI_HitStop.StartHitStop` _asbp_player)
            (set `local.TriggeredShake` true))
          (`KismetArrayLibrary.Array_Add` _hitactors _returnvalue)
          (bind _ascontroller (cast `Controller` _returnvalue))
          (`/Engine/EditorBlueprintResources/StandardMacros.IsValid` _ascontroller
            (:`Is Valid`
              (bind _output_get (set `self.AttackTarget` (`Controller.K2_GetPawn` _ascontroller)))
              (bind _didhit (`self.HitResponse` _output_get))
              (if _didhit
                (`AbilitySystemComponent.BP_ApplyGameplayEffectToTarget` :`self` (`AbilitySystemBlueprintLibrary.GetAbilitySystemComponent` (`self.GetAvatarActorFromActorInfo`)) :`GameplayEffectClass` "/Game/MyContent/Blueprints/GameplayEffect/GE_PhysicalDamage.GE_PhysicalDamage_C" :`Target` (`AbilitySystemBlueprintLibrary.GetAbilitySystemComponent` _output_get))
                (`self.ApplyPoiseDamage`)
                (else
                  (`KismetSystemLibrary.PrintString` "Couldn't hit"))))))))))

(fn `WasInterrupted`
  (returns (WasInterrupted :type Boolean))
  (return (`GameplayTagAssetInterface.HasAnyMatchingGameplayTags` (`AbilitySystemBlueprintLibrary.GetAbilitySystemComponent` (`self.GetAvatarActorFromActorInfo`)) (`self.InterruptTags`))))