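; Generic attack gameplay ability that instantly damages whatever stands in a box in front of the avatar.
; On successful commit it runs a debug-drawn multi box trace ahead of the avatar, sized by the attack data's hitbox scale, then ends.
; Each hit actor's owner is recorded to skip repeats, and new hits receive GE_Damage, with debug prints for both cases.
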(event `self.K2_ActivateAbility`
  (bind _returnvalue (`self.K2_CommitAbility`))
  (if _returnvalue
    (bind _outhits (`self.HitZoneScan` (`Skill.HitBoxScale` (`self.AttackData`))))
    (`self.ProcessHits` _outhits)
    (`self.K2_EndAbility`)
    (else
      (`self.K2_CancelAbility`))))

(fn `HitZoneScan`
  (params (HitBoxScale :type "Vector Structure"))
  (returns (OutHits :type "Array of HitResult Structure"))
  (bind _returnvalue (`self.GetAvatarActorFromActorInfo`))
  (bind _returnvalue_2 (+ (`Actor.K2_GetActorLocation` _returnvalue) (* 100.0 (`Actor.GetActorForwardVector` _returnvalue))))
  (bind _outhits (`KismetSystemLibrary.BoxTraceMulti` _returnvalue_2 (+ _returnvalue_2 (0.1 0.1 0.1)) (* HitBoxScale (32.0 32.0 32.0)) (`Actor.K2_GetActorRotation` _returnvalue) "TraceTypeQuery3" false (`|MakeArray` _returnvalue) "ForDuration"))
  (return _outhits))

(fn `ProcessHits`
  (params (Array :type "Array of HitResult Structure"))
  (bind _array (`|MakeArray` null :!type "Actor Object Reference"))
  (for (_array_element _array_index) Array
    (bind (_bblockinghit _binitialoverlap _time _distance _location _impactpoint _normal _impactnormal _physmat _hitactor) (`GameplayStatics.BreakHitResult` _array_element))
    (bind _returnvalue (`Actor.GetOwner` _hitactor))
    (if (`KismetArrayLibrary.Array_Contains` _array _returnvalue)
      (`KismetSystemLibrary.PrintString` "Already hit this target")
      (else
        (`KismetArrayLibrary.Array_Add` _array _returnvalue)
        (`KismetSystemLibrary.PrintString` (`KismetStringLibrary.Conv_IntToString` _array_index))
        (`self.BP_ApplyGameplayEffectToTarget` (`AbilitySystemBlueprintLibrary.AbilityTargetDataFromActor` _hitactor) "/Game/MyContent/Blueprints/GameplayEffect/GE_Damage.GE_Damage_C")))))