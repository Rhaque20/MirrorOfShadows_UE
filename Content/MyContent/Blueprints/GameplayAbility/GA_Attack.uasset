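; GA_Attack is a Gameplay Ability that performs a short-range melee-style attack in front of the avatar.
; On activation it commits, then runs a multi sphere trace for Pawn objects along the avatar's forward vector, ignoring the avatar.
; Each hit prints its component name and receives GE_Damage through target data built from the hit actor, with debug trace drawing enabled.
; The ability ends after processing hits, or cancels if the commit fails.
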(event `self.K2_ActivateAbility`
  (bind _returnvalue (`self.GetAvatarActorFromActorInfo`))
  (bind _returnvalue_2 (`Actor.K2_GetActorLocation` _returnvalue))
  (bind _returnvalue_3 (`self.K2_CommitAbility`))
  (if _returnvalue_3
    (bind _outhits (`KismetSystemLibrary.SphereTraceMultiForObjects` _returnvalue_2 (+ _returnvalue_2 (* (`Actor.GetActorForwardVector` _returnvalue) 100.0)) 50.0 (`|MakeArray` "ObjectTypeQuery3" :!type "EObjectTypeQuery Enum") false (`|MakeArray` _returnvalue) "ForDuration"))
    (for _array_element _outhits
      (bind (_bblockinghit _binitialoverlap _time _distance _location _impactpoint _normal _impactnormal _physmat _hitactor _hitcomponent) (`GameplayStatics.BreakHitResult` _array_element))
      (`KismetSystemLibrary.PrintString` (`KismetSystemLibrary.GetDisplayName` _hitcomponent))
      (`self.BP_ApplyGameplayEffectToTarget` (`AbilitySystemBlueprintLibrary.AbilityTargetDataFromActor` _hitactor) "/Game/MyContent/Blueprints/GameplayEffect/GE_Damage.GE_Damage_C"))
    (`self.K2_EndAbility`)
    (else
      (`self.K2_CancelAbility`))))