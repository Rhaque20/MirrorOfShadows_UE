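; GA_DodgeRoll is an event-activated gameplay ability that makes an RPG character dodge roll using the montage passed in the event payload.
; After committing, it applies an evade effect with a set-by-caller magnitude for i-frames plus a perfect-dodge window effect to the avatar.
; It calls PerformDodge and locks movement until a melee recover event or ability end.
; An interrupted or cancelled montage calls CancelDodge before ending the ability.
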(event `self.K2_OnEndAbility`
  (params (bWasCancelled :type Boolean))
  (set `RPGCharacterBase.CanMove` true (`self.AbilityOwner`)))

(event `self.K2_ActivateAbilityFromEvent`
  (params (EventData :type "GameplayEventData Structure (by ref)"))
  (bind _returnvalue (`AbilitySystemBlueprintLibrary.GetAbilitySystemComponent` (`self.GetAvatarActorFromActorInfo`)))
  (bind _returnvalue_2 (`self.K2_CommitAbility`))
  (if _returnvalue_2
    (bind _asanim_montage (cast `AnimMontage` (`.OptionalObject` (break `GameplayEventData` EventData))))
    ;[1 1 1] Apply both Iframe and Perfect Dodge window effect to caster
    (bind _returnvalue_3 (`AbilitySystemBlueprintLibrary.AssignTagSetByCallerMagnitude` (`AbilitySystemComponent.MakeOutgoingSpec` :`self` _returnvalue :`GameplayEffectClass` "/Game/MyContent/Blueprints/GameplayEffect/GE_Evade.GE_Evade_C") (struct :`TagName` "Effect.Defensive.Evade") 0.5))
    (`AbilitySystemComponent.BP_ApplyGameplayEffectSpecToSelf` _returnvalue _returnvalue_3)
    (`AbilitySystemComponent.BP_ApplyGameplayEffectToSelf` :`self` _returnvalue :`GameplayEffectClass` "/Game/MyContent/Blueprints/GameplayEffect/GE_PerfectDodge.GE_PerfectDodge_C")
    (`AbilityTask_PlayMontageAndWait.CreatePlayMontageAndWaitProxy` "None" _asanim_montage
      (:`then`
        (bind _asrpgcharacter_base (cast `RPGCharacterBase` (`self.GetAvatarActorFromActorInfo`)))
        (`RPGCharacterBase.PerformDodge` _asrpgcharacter_base)
        (set `self.AbilityOwner` _asrpgcharacter_base)
        (set `RPGCharacterBase.CanMove` false _asrpgcharacter_base)
        (`AbilityTask_WaitGameplayEvent.WaitGameplayEvent` (struct :`TagName` "Event.Melee.Recover") null
          (:`EventReceived`
            (set `RPGCharacterBase.CanMove` true _asrpgcharacter_base))))
      (:`OnCompleted`
        (`self.K2_EndAbility` :!label _label))
      (:`OnBlendOut`
        (goto _label))
      (:`OnInterrupted`
        (`RPGCharacterBase.CancelDodge` _asrpgcharacter_base :!label _label_2)
        (`RPGCharacterBase.CancelDodge` (`self.AbilityOwner`))
        (goto _label))
      (:`OnCancelled`
        (goto _label_2)))
    (else
      (`self.K2_EndAbility`))))