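; Hit reaction gameplay ability that plays a block or stagger montage on an RPGCharacterBase avatar.
; A Block tag plays the BlockSuccess section without ending the ability; otherwise PoiseBroken triggers the StaggerComponent's light stagger.
; The non-block path ends immediately, letting the stagger montage continue past the ability.
; Ending the ability removes effects granting the NormalAttack input tag.
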(event `self.K2_OnEndAbility`
  (params (bWasCancelled :type Boolean))
  (`AbilitySystemComponent.RemoveActiveEffectsWithGrantedTags` (`AbilitySystemBlueprintLibrary.GetAbilitySystemComponent` (`self.GetAvatarActorFromActorInfo`)) (struct :`GameplayTags` (struct :`(TagName` "Ability.Input.NormalAttack") :`(TagName` "Ability.Input.Skill"))))
  (`KismetSystemLibrary.PrintString` "Hit React End"))

(event `self.K2_ActivateAbility`
  (bind _returnvalue (`AbilitySystemBlueprintLibrary.GetAbilitySystemComponent` (`self.GetAvatarActorFromActorInfo`)))
  ;[1 1 1] Get stagger animation from stagger component
  (bind _asrpgcharacter_base (cast `RPGCharacterBase` (`self.GetAvatarActorFromActorInfo`))
    (:`then`
      (set `self.RegularStagger` (`StaggerComponent.LightStaggerAnim` (`RPGCharacterBase.StaggerComponent` _asrpgcharacter_base)))
      (if (`GameplayTagAssetInterface.HasMatchingGameplayTag` _returnvalue (struct :`TagName` "Effect.Defensive.Block"))
        (`|PlayMontage` (`self.GetOwningComponentFromActorInfo`) (`self.BlockStagger`) 1.0 0.0 "BlockSuccess"
          (:`then`
            _))
        (elif (`GameplayTagAssetInterface.HasMatchingGameplayTag` _returnvalue (struct :`TagName` "Effect.State.PoiseBroken"))
          (`AbilityTask_PlayMontageAndWait.CreatePlayMontageAndWaitProxy` "None" (`self.RegularStagger`) 1.0 "Default" false
            (:`then`
              _))))
      (`self.K2_EndAbility`))
    (:`CastFailed`
      (`KismetSystemLibrary.PrintString` "Does not inherit from character base"))))