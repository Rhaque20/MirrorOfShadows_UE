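; BP_EnemyBase is the base enemy character, using the Gameplay Ability System for combat, with wolf-specific test attacks and death.
; BeginPlay grants abilities and effects and initializes a camera-facing, distance-limited status widget; sight sets the AI blackboard's target and combat state.
; Bite, claw and dodge functions activate abilities, then drive velocity through a curve-based launch timeline.
; Damage spawns floating numbers; death releases lock-on, plays a montage and destroys the actor.
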(event `self.DisplayDamageNumber`
  (params (Container :type "GameplayTagContainer Structure (by ref)") (Damage :type "Float (single-precision)") (DidHit :type Integer))
  (for _array_element (`BlueprintGameplayTagLibrary.BreakGameplayTagContainer` Container)
    (if (`BlueprintGameplayTagLibrary.MatchesTag` _array_element (struct :`TagName` "Damage.Health"))
      (`|SwitchGameplayTag` _array_element
        (:`Damage.Health.Light`
          (`KismetSystemLibrary.PrintString` "Taken Light Damage")
          (break))
        (:`Damage.Health.Physical`
          (`KismetSystemLibrary.PrintString` "Taken Physical Damage")
          (break))))))

(event `self.ReceiveAnyDamage`
  (params (Damage :type "Float (single-precision)") (DamageType :type "DamageType Object Reference") (InstigatedBy :type "Controller Object Reference") (DamageCauser :type "Actor Object Reference"))
  (`|SpawnActorFromClass` "/Game/MyContent/Blueprints/UI/CombatUI/BP_DamageNumber.BP_DamageNumber_C" (`self.GetTransform`) "Undefined" "MultiplyWithRoot" null Damage (`self.K2_GetActorLocation`) null))

(event `self.ReceiveBeginPlay`
  (bind _abilitysystem (`self.AbilitySystem`))
  (`self.AbilityGranting`)
  (set `self.HurtboxLocation` (`SceneComponent.RelativeLocation` (`self.HurtboxSpot`)))
  (bind _aswbp_enemy_status (cast `/Game/MyContent/Blueprints/UI/CombatUI/WBP_EnemyStatus` (`WidgetComponent.GetWidget` (`self.Status`))))
  (`/Game/MyContent/Blueprints/UI/CombatUI/WBP_EnemyStatus.SettingUp` _aswbp_enemy_status self)
  (`/Game/MyContent/Blueprints/UI/CombatUI/WBP_EnemyStatus.Update Health Bar Main` _aswbp_enemy_status (`.ReturnValue` (`AbilitySystemComponent.GetGameplayAttributeValue` _abilitysystem (struct :`AttributeName` "CurrentHP" :`Attribute` "/Script/MirrorOfShadows.BaseAttributeSet:CurrentHP" :`AttributeOwner` "/Script/CoreUObject.Class'/Script/MirrorOfShadows.BaseAttributeSet'"))) (`.ReturnValue` (`AbilitySystemComponent.GetGameplayAttributeValue` _abilitysystem (struct :`AttributeName` "TotalHP" :`Attribute` "/Script/MirrorOfShadows.BaseAttributeSet:TotalHP" :`AttributeOwner` "/Script/CoreUObject.Class'/Script/MirrorOfShadows.BaseAttributeSet'"))))
  (set `self.StaggerComponent` (`self.EnemyStaggerCore`))
  (set `self.AttackTarget` (`GameplayStatics.GetPlayerPawn` 0))
  (`AbilitySystemComponent.BP_ApplyGameplayEffectToSelf` :`self` (`self.AbilitySystem`) :`GameplayEffectClass` "/Game/MyContent/Blueprints/GameplayEffect/Cooldowns/Enemy/GE_EvadeCharge.GE_EvadeCharge_C"))

(event `self.ReceiveTick`
  (params (DeltaSeconds :type "Float (single-precision)"))
  (`self.DisplayHealthBar`)
  (`self.Update Health Bar`))

(event `self.OnDeath`
  (bind _abilitysystem (`self.AbilitySystem`))
  (if (not (`GameplayTagAssetInterface.HasMatchingGameplayTag` _abilitysystem (struct :`TagName` "Effect.State.Dead")))
    (`KismetSystemLibrary.PrintString` "WolfDead")
    (`PrimitiveComponent.SetCollisionEnabled` (`self.CapsuleComponent`) "NoCollision")
    (bind _asbp_character_controller (cast `/Game/MyContent/Blueprints/Character_BP/BP_CharacterController` (`GameplayStatics.GetPlayerController` 0)))
    (`/Engine/EditorBlueprintResources/StandardMacros.IsValid` _asbp_character_controller
      (:`Is Valid`
        (`/Game/MyContent/Blueprints/Character_BP/BP_CharacterController.CheckIfLockedOnTest` _asbp_character_controller self))
      (:`Is Not Valid`
        _))
    (`self.StopAnimMontage` null)
    (`AbilitySystemComponent.BP_ApplyGameplayEffectToSelf` :`self` _abilitysystem :`GameplayEffectClass` "/Game/MyContent/Blueprints/GameplayEffect/GE_Dead.GE_Dead_C")
    (`|PlayMontage` (`self.Mesh`) "/Game/MyContent/Animations/Enemy/SilverWolfAnim/SilverWolfMontage/Wolf_Death.Wolf_Death"
      (:`then`
        (`KismetSystemLibrary.Delay` 0.6)
        (`self.K2_DestroyActor`)))))

(event `self.PawnSensing.OnSeePawn`
  (params (Pawn :type "Pawn Object Reference"))
  (bind _returnvalue (`AIBlueprintHelperLibrary.GetAIController` self))
  (bind _returnvalue_2 (`AIBlueprintHelperLibrary.GetBlackboard` _returnvalue))
  (`/Engine/EditorBlueprintResources/StandardMacros.IsValid` (`AIBlueprintHelperLibrary.GetBlackboard` (`AIBlueprintHelperLibrary.GetAIController` null))
    (:`Is Valid`
      (bind _output_get (set `self.AttackTarget` Pawn))
      (if (not (`self.SpotsPlayer`))
        (set `self.SpotsPlayer` true)
        (`KismetSystemLibrary.PrintString` (`KismetStringLibrary.Concat_StrStr` "Spotted " (`KismetSystemLibrary.GetDisplayName` _output_get)))
        (bind _asbp_enemy_aicontroller (cast `/Game/MyContent/Blueprints/Enemy_BP/BP_EnemyAIController` _returnvalue))
        (set `EnemyAIController.PlayerPawn` Pawn _asbp_enemy_aicontroller)
        (`BlackboardComponent.SetValueAsObject` _returnvalue_2 "Target" _output_get)
        (`BlackboardComponent.SetValueAsBool` _returnvalue_2 "InCombat" true)
        (`NavMovementComponent.StopActiveMovement` (`self.CharacterMovement`))))))

(event `StartLaunch`
  (bind _charactermovement (`self.CharacterMovement`))
  (bind _activeskill (`self.ActiveSkill`))
  (bind (_velocity_x _velocity_y _velocity_z) (`KismetMathLibrary.BreakVector` (`MovementComponent.Velocity` _charactermovement)))
  (`TimelineComponent.SetTimelineLength` (`self.LaunchTimeline`) (`AnimationAsset.GetPlayLength` (`Skill.GetAnimation` _activeskill 0)))
  (bind (_direction _timedelta) (`Timeline|LaunchTimeline` :!via `PlayFromStart`)
    (:`Update`
      (bind (_returnvalue_x _returnvalue_y) (`KismetMathLibrary.BreakVector` (* (`self.GetActorForwardVector`) (* (`CurveFloat.GetFloatValue` (`Skill.LaunchCurve` _activeskill) _timedelta) (`KismetSystemLibrary.MakeLiteralDouble` (`Skill.LaunchForce` _activeskill))))))
      (set `MovementComponent.Velocity` (`KismetMathLibrary.MakeVector` _returnvalue_x _returnvalue_y _velocity_z) _charactermovement))))

(event `EndLaunch`
  (`TimelineComponent.Stop` (`self.LaunchTimeline`))
  (`self.Recover`))

(event `self.K2_OnMovementModeChanged`
  (params (PrevMovementMode :type "EMovementMode Enum" :default "MOVE_None") (NewMovementMode :type "EMovementMode Enum" :default "MOVE_None") (PrevCustomMode :type Byte) (NewCustomMode :type Byte))
  (`KismetSystemLibrary.PrintString` (`KismetStringLibrary.Concat_StrStr` "Movement mode changed from: " (`KismetStringLibrary.Conv_ByteToString` PrevMovementMode) " to " (`KismetStringLibrary.Conv_ByteToString` NewMovementMode))))

(event `FollowPlayer`
  (params (Pawn :type "Pawn Object Reference"))
  (if (and (`self.SpotsPlayer`) (`self.CanMove`))
    (`|AIMoveTo` self (0.0 0.0 0.0) Pawn 150.0 true
      (:`OnSuccess`
        (bind _success (`self.Test Wolf Bite`))
        (if _success
          _
          (elif (not (`GameplayTagAssetInterface.HasAnyMatchingGameplayTags` (`self.AbilitySystem`) (`BlueprintGameplayTagLibrary.MakeLiteralGameplayTagContainer` (struct :`GameplayTags` (struct :`(TagName` "Effect.Defensive.Evade") :`(TagName` "Effect.State"))))))
            (set `self.CanMove` true)
            (set `self.IsAttacking` false)))))))

(event `/Game/MyContent/InterfaceBlueprints/BPI_HitStop.StartHitStop`)

(fn `AbilityGranting`
  (bind _abilitysystem (`self.AbilitySystem`))
  (for _array_element (`self.AbilityListTest`)
    (`AbilitySystemComponent.K2_GiveAbility` _abilitysystem _array_element 0 -1))
  (`AbilitySystemComponent.BP_ApplyGameplayEffectToSelf` :`self` _abilitysystem :`GameplayEffectClass` "/Game/MyContent/Blueprints/GameplayEffect/PoiseSystem/GE_PoiseDrain.GE_PoiseDrain_C"))

(fn `AimAtPlayer`
  (bind (_returnvalue_roll _returnvalue_pitch) (`KismetMathLibrary.BreakRotator` (`self.K2_GetActorRotation`)))
  (bind (_returnvalue_roll_2 _returnvalue_pitch_2 _returnvalue_yaw) (`KismetMathLibrary.BreakRotator` (`KismetMathLibrary.FindLookAtRotation` (`self.K2_GetActorLocation`) (`self.K2_GetActorLocation` (`self.AttackTarget`)))))
  (`self.K2_SetActorRotation` (`KismetMathLibrary.MakeRotator` _returnvalue_roll _returnvalue_pitch _returnvalue_yaw)))

(fn `DisplayHealthBar`
  (`SceneComponent.SetVisibility` (`self.Status`) (and (<= (`KismetMathLibrary.Vector_Distance` (`self.K2_GetActorLocation`) (`self.K2_GetActorLocation` (`GameplayStatics.GetPlayerPawn` 0))) (`self.MaxStatusDisplayDistance`)) (not (`GameplayTagAssetInterface.HasMatchingGameplayTag` (`self.AbilitySystem`) (struct :`TagName` "Effect.State.Dead")))) false))

(fn `SetHurtboxSpot`
  (params (NewSpot :type "Vector Structure"))
  (returns (HurtboxSpot :type "Vector Structure") (FinalHurtboxSpot :type "Vector Structure"))
  (locals (StartSpot :type "Vector Structure") (FinalSpot :type "Vector Structure"))
  (bind _hurtboxspot (`self.HurtboxSpot`))
  (bind _returnvalue (`SceneComponent.K2_GetComponentLocation` _hurtboxspot))
  (`SceneComponent.K2_SetRelativeLocation` _hurtboxspot (+ NewSpot (`self.HurtboxLocation`)) false false)
  (bind _output_get (set `local.StartSpot` _returnvalue))
  (bind _output_get_2 (set `local.FinalSpot` _returnvalue))
  (return _output_get _output_get_2))

(fn `Test Wolf Bite`
  (returns (Success :type Boolean))
  (locals (SkillSuccess :type Boolean))
  (bind _returnvalue (`AbilitySystemBlueprintLibrary.GetAbilitySystemComponent` null))
  (bind _moveset (`self.Moveset`))
  (bind _aspawn (cast `Pawn` (`self.AttackTarget`)))
  (if (and (<= (`self.GetConditionParameters` _aspawn) 300.0) (not (`GameplayTagAssetInterface.HasAnyMatchingGameplayTags` (`self.AbilitySystem`) (`BlueprintGameplayTagLibrary.MakeLiteralGameplayTagContainer` (struct :`GameplayTags` (struct :`(TagName` "Effect.Defensive.Evade") :`(TagName` "Effect.State")))))))
    (set `self.IsAttacking` true)
    (set `self.CanMove` false)
    (if (`GameplayTagAssetInterface.HasMatchingGameplayTag` _returnvalue (struct :`TagName` "Skill.Cooldown.Enemy.Regular.Skill1"))
      (set `self.ActiveSkill` (`|GetArrayItem` _moveset))
      (bind _returnvalue_2 (`AbilitySystemComponent.TryActivateAbilityByClass` (`self.AbilitySystem`) "/Game/MyContent/Blueprints/GameplayAbility/EnemyAbilities/Wolf/GA_WolfBite.GA_WolfBite_C" true))
      (set `local.SkillSuccess` _returnvalue_2)
      (else
        (set `self.ActiveSkill` (`|GetArrayItem` _moveset 1))
        (`KismetSystemLibrary.PrintString` "Claw strike")
        (bind _returnvalue_3 (`AbilitySystemComponent.TryActivateAbilityByClass` _returnvalue "/Game/MyContent/Blueprints/GameplayAbility/EnemyAbilities/Wolf/GA_ClawStrike.GA_ClawStrike_C" true))
        (set `local.SkillSuccess` _returnvalue_3)))
    (if (`local.SkillSuccess`)
      (`self.AimAtPlayer`)
      (`self.StartLaunch`)
      (else
        (`self.Recover`)
        (`KismetSystemLibrary.PrintString` "Call ability failed")))
    (return (`local.SkillSuccess`))
    (else
      (return false))))

(fn `TestEvade`
  (returns (Successful :type Boolean))
  (bind _charactermovement (`self.CharacterMovement`))
  (bind _returnvalue (`AbilitySystemComponent.TryActivateAbilityByClass` (`AbilitySystemBlueprintLibrary.GetAbilitySystemComponent` null) "/Game/MyContent/Blueprints/GameplayAbility/EnemyAbilities/Wolf/GA_EnemyDodge.GA_EnemyDodge_C" true))
  (if _returnvalue
    (set `self.ActiveSkill` (`|GetArrayItem` (`self.Moveset`) 2))
    (`MovementComponent.StopMovementImmediately` _charactermovement)
    (`NavMovementComponent.StopActiveMovement` _charactermovement)
    (set `self.CanMove` false)
    (`KismetSystemLibrary.PrintString` "Start evade launch")
    (`self.AimAtPlayer`)
    (`self.StartLaunch`))
  (return _returnvalue))

(fn `Update Health Bar`
  (bind _status (`self.Status`))
  (`SceneComponent.K2_SetWorldRotation` _status (`KismetMathLibrary.FindLookAtRotation` (`SceneComponent.K2_GetComponentLocation` _status) (`SceneComponent.K2_GetComponentLocation` (`PlayerCameraManager.TransformComponent` (`GameplayStatics.GetPlayerCameraManager` 0)))) false false))

(fn `UserConstructionScript`)