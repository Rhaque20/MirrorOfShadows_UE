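; Flying enemy base that wanders between random points until PawnSensing spots a pawn, then switches to chasing the player.
; Wander points come from random offsets checked by line traces, with a new one chosen on arrival.
; Tick sets CharacterMovement velocity directly, closing horizontally on the player to a standoff distance.
; During pursuit, it seeks hover height above the GameMode's ground elevation, climbing steadily whenever its visibility trace misses the player.
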(event `self.ReceiveBeginPlay`
  (`parent.ReceiveBeginPlay`)
  (set `self.AttackTarget` (`GameplayStatics.GetPlayerCharacter` 0))
  (bind _asbp_combat_game_mode (cast `/Game/MyContent/Blueprints/GameModes/BP_CombatGameMode` (`GameplayStatics.GetGameMode`)))
  (set `self.GameModeRef` _asbp_combat_game_mode)
  (bind _wanderspot (`self.GenerateWanderSpot`))
  (set `self.WanderSpotCache` _wanderspot))

(event `self.ReceiveTick`
  (params (DeltaSeconds :type "Float (single-precision)"))
  (`parent.ReceiveTick` DeltaSeconds)
  (if (`self.ActivelyWander`)
    (`self.FlyingMovement2` (`self.WanderSpotCache`))
    (else
      (`self.AimAtPlayer`)
      (`self.FlyingMovement`))))

(event `self.PawnSensing.OnSeePawn`
  (params (Pawn :type "Pawn Object Reference"))
  (if (`self.ActivelyWander`)
    (set `MovementComponent.Velocity` (0.0 0.0 0.0) (`self.CharacterMovement`)))
  (set `self.ActivelyWander` false))

(fn `CanReachPlayerAtHeight`
  (returns (CanReach :type Boolean))
  (bind _outhit (`KismetSystemLibrary.LineTraceSingle` :`Start` (`self.K2_GetActorLocation` self) :`End` (`self.K2_GetActorLocation` (`self.AttackTarget`)) :`TraceChannel` "TraceTypeQuery1" :`DrawTime` 1.0))
  (return (== (`.HitActor` (`GameplayStatics.BreakHitResult` _outhit)) (`self.AttackTarget`))))

(fn `FlyingMovement`
  (bind (_returnvalue_x _returnvalue_y _returnvalue_z) (`KismetMathLibrary.BreakVector` (`self.K2_GetActorLocation`)))
  (bind (_returnvalue_x_2 _returnvalue_y_2 _returnvalue_z_2) (`KismetMathLibrary.BreakVector` (`self.K2_GetActorLocation`)))
  (bind (_returnvalue_x_3 _returnvalue_y_3 _returnvalue_z_3) (`KismetMathLibrary.BreakVector` (`self.K2_GetActorLocation`)))
  (bind _canreach (`self.CanReachPlayerAtHeight`))
  (bind _charactermovement (`self.CharacterMovement`))
  (bind _charactermovement_2 (`self.CharacterMovement`))
  (bind _charactermovement_3 (`self.CharacterMovement`))
  (bind (_returnvalue_x_4 _returnvalue_y_4) (`KismetMathLibrary.BreakVector` (* (`self.GetActorForwardVector`) 200.0)))
  (bind (_velocity_x _velocity_y) (`KismetMathLibrary.BreakVector` (`MovementComponent.Velocity` _charactermovement)))
  (bind (_velocity_x_2 _velocity_y_2 _velocity_z) (`KismetMathLibrary.BreakVector` (`MovementComponent.Velocity` _charactermovement_2)))
  (bind (_velocity_x_3 _velocity_y_3) (`KismetMathLibrary.BreakVector` (`MovementComponent.Velocity` _charactermovement_3)))
  (bind _returnvalue (+ (`/Game/MyContent/Blueprints/GameModes/BP_CombatGameMode.GroundElevation` (`self.GameModeRef`)) (`self.MaxHoverHeight`)))
  (`|ExecutionSequence`
    (:`then_0`
      ;[1 1 1] Move towards target when too far away
      (if (> (`KismetMathLibrary.Vector_Distance2D` (`self.K2_GetActorLocation`) (`self.K2_GetActorLocation` (`GameplayStatics.GetPlayerCharacter` 0))) 200.0)
        (set `MovementComponent.Velocity` (`KismetMathLibrary.MakeVector` _returnvalue_x_4 _returnvalue_y_4 _velocity_z) _charactermovement_2)
        (else
          (set `MovementComponent.Velocity` (`KismetMathLibrary.MakeVector` 0.0 0.0 _velocity_z) _charactermovement_2))))
    (:`then_1`
      (if (and (< _returnvalue_z _returnvalue) _canreach)
        ;[1 1 1] When in view of player and not at the max height.
        (set `MovementComponent.Velocity` (`KismetMathLibrary.MakeVector` _velocity_x_3 _velocity_y_3 (- _returnvalue _returnvalue_z_3)) _charactermovement_3)
        (elif _canreach
          (set `MovementComponent.Velocity` (`KismetMathLibrary.MakeVector` _velocity_x _velocity_y (- _returnvalue _returnvalue_z_2)) _charactermovement)
          (else
            (set `MovementComponent.Velocity` (`KismetMathLibrary.MakeVector` _velocity_x _velocity_y 50.0) _charactermovement)))))))

(fn `FlyingMovement2`
  (params (FlyLocation :type "Vector Structure"))
  (bind (_returnvalue_roll _returnvalue_pitch) (`KismetMathLibrary.BreakRotator` (`self.K2_GetActorRotation`)))
  (bind _charactermovement (`self.CharacterMovement`))
  (bind _returnvalue (`self.K2_GetActorLocation` self))
  (bind (_returnvalue_roll_2 _returnvalue_pitch_2 _returnvalue_yaw) (`KismetMathLibrary.BreakRotator` (`KismetMathLibrary.FindLookAtRotation` _returnvalue FlyLocation)))
  (bind _returnvalue_2 (`KismetMathLibrary.Vector_Distance` _returnvalue FlyLocation))
  (if (> _returnvalue_2 (`self.PointProximity`))
    (`self.K2_SetActorRotation` (`KismetMathLibrary.MakeRotator` _returnvalue_roll _returnvalue_pitch _returnvalue_yaw))
    (set `MovementComponent.Velocity` (* (`self.GetActorForwardVector`) 250.0) _charactermovement)
    (else
      (set `MovementComponent.Velocity` (0.0 0.0 0.0) _charactermovement)
      (`KismetSystemLibrary.PrintText` (`|FormatText` "Distance is {distance}" _returnvalue_2))
      (bind _wanderspot (`self.GenerateWanderSpot`))
      (set `self.WanderSpotCache` _wanderspot))))

(fn `GenerateWanderSpot`
  (returns (WanderSpot :type "Vector Structure"))
  (locals (WanderDistance :type "Float (double-precision)" :default 500.0) (StillSearching :type Boolean :default true) (WanderPos :type "Vector Structure"))
  (bind (_returnvalue_x _returnvalue_y _returnvalue_z) (`KismetMathLibrary.BreakVector` (`SceneComponent.K2_GetComponentLocation` (`self.CapsuleComponent`))))
  (while (`local.StillSearching`)
    (bind _output_get (set `local.WanderPos` (`KismetMathLibrary.MakeVector` (+ _returnvalue_x (* (`KismetMathLibrary.RandomFloatInRange` -2.0 2.0) (`local.WanderDistance`))) (+ (* (`KismetMathLibrary.RandomFloatInRange` -2.0 2.0) (`local.WanderDistance`)) _returnvalue_y) _returnvalue_z)))
    (bind (_outhit _returnvalue) (`KismetSystemLibrary.LineTraceSingle` (`SceneComponent.K2_GetComponentLocation` (`self.CapsuleComponent`)) _output_get "TraceTypeQuery1"))
    (if _returnvalue
      (bind (_bblockinghit _binitialoverlap _time _distance _location _impactpoint) (`GameplayStatics.BreakHitResult` _outhit))
      (bind _output_get_2 (set `local.StillSearching` (not (>= (`KismetMathLibrary.Vector_Distance2D` _impactpoint (`self.K2_GetActorLocation`)) 50.0))))
      (if (not _output_get_2)
        (set `local.WanderPos` _impactpoint))
      (else
        (set `local.StillSearching` _returnvalue))))
  (return (`local.WanderPos`)))

(fn `UserConstructionScript`
  (`parent.UserConstructionScript`))