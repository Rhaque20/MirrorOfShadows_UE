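; BP_HitScan is an animation notify state that, despite its name, manages the player's attack recovery and combo window without performing any trace.
; On begin, it calls Recover on the CharacterCore of player 0's PlayerCharacters, not the mesh's owner.
; On end, it resets CurrentChain to zero unless IsAttacking is set, which lets the chain continue.
; Both events print debug strings.
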(fn `Received_NotifyBegin`
  (params (MeshComp :type "SkeletalMeshComponent Object Reference") (Animation :type "AnimSequenceBase Object Reference") (TotalDuration :type "Float (single-precision)") (EventReference :type "AnimNotifyEventReference Structure (by ref)"))
  (returns (ReturnValue :type Boolean))
  (bind _asplayer_characters (cast `PlayerCharacters` (`GameplayStatics.GetPlayerCharacter` MeshComp)))
  (`PlayerCore.Recover` (`CecilePlayable.CharacterCore` _asplayer_characters))
  (`KismetSystemLibrary.PrintString` MeshComp "In Recovery State")
  (return false))

(fn `Received_NotifyEnd`
  (params (MeshComp :type "SkeletalMeshComponent Object Reference") (Animation :type "AnimSequenceBase Object Reference") (EventReference :type "AnimNotifyEventReference Structure (by ref)"))
  (returns (ReturnValue :type Boolean))
  (bind _asplayer_characters (cast `PlayerCharacters` (`GameplayStatics.GetPlayerCharacter` MeshComp)))
  (bind _charactercore (`CecilePlayable.CharacterCore` _asplayer_characters))
  (if (`CombatComponent.bIsAttacking` _charactercore)
    (`KismetSystemLibrary.PrintString` null "Continuing Attack")
    (else
      (set `PlayerCore.CurrentChain` 0 _charactercore)
      (`KismetSystemLibrary.PrintString` MeshComp "End of Notify Attack")))
  (return false))