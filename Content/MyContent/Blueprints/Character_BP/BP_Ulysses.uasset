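; BP_Ulysses is a character Blueprint with ground and air state tracking and an unfinished normal-attack combo.
; Tick stores whether the movement component is on the ground and, when airborne, the sign of the capsule's vertical physics velocity.
; SomethingFunny looks up the current chain's attack montage in CharacterCore, with debug prints.
; Its montage playback is disconnected, and the IA_NormalAttack input event does nothing.
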(event `self.ReceiveTick`
  (params (DeltaSeconds :type "Float (single-precision)"))
  (bind _output_get (set `self.OnGround` (`NavMovementComponent.IsMovingOnGround` (`self.CharacterMovement`))))
  (if (not _output_get)
    (bind _returnvalue (`PrimitiveComponent.GetPhysicsLinearVelocity` (`self.CapsuleComponent`) "None"))
    (set `self.AerialVelocity` (`KismetMathLibrary.SignOfFloat` (.z _returnvalue)))))

(event `EnhancedInput|/Game/MyContent/InputActions/IA_NormalAttack`
  (params (ActionValue :type Boolean) (ElapsedSeconds :type "Float (double-precision)") (TriggeredSeconds :type "Float (double-precision)") (InputAction :type "InputAction Object Reference" :default "/Game/MyContent/InputActions/IA_NormalAttack.IA_NormalAttack")))

(fn `SomethingFunny`
  (returns (Mesh :type "SkeletalMeshComponent Object Reference") (`AsAnim Montage` :type "AnimMontage Object Reference"))
  (bind _charactercore (`self.CharacterCore`))
  (bind _currentchain (`PlayerCore.CurrentChain` _charactercore))
  (bind _normalattacks (`PlayerCore.NormalAttacks` _charactercore))
  (if (`KismetArrayLibrary.Array_IsValidIndex` _normalattacks _currentchain)
    (`KismetSystemLibrary.PrintString` (`KismetStringLibrary.Conv_IntToString` _currentchain))
    (return (`self.Mesh`) (`Skill.GetAnimation` (`|GetArrayItem` _normalattacks _currentchain) 0))
    (else
      (`KismetSystemLibrary.PrintString` "Invalid Access"))))

(fn `UserConstructionScript`)