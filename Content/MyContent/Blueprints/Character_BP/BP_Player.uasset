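; Player character that drives normal attacks and skills through the Gameplay Ability System, with attack buffering and lock-on facing.
; On BeginPlay it grants both abilities and turns equipped gear stats into SetByCaller gameplay effects, currently handling only helmets and flat HP main stats.
; Hit stop briefly slows the actor and its tracked slash VFX through custom time dilation.
; Damage taken spawns damage numbers, and a debug key removes helmet effects.
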(event Input|EnhancedActionEvents|EnhancedInputActionIA_NormalAttack
  (params (ActionValue :type Boolean) (ElapsedSeconds :type Float%20%28double-precision%29) (TriggeredSeconds :type Float%20%28double-precision%29) (InputAction :type Input%20Action%20Object%20Reference :default "/Game/MyContent/InputActions/IA_NormalAttack.IA_NormalAttack"))
  (bind _charactercore (Variables|Default|GetCharacterCore))
  (:Started
    (Development|PrintString "Exceuting Normal")
    (bind _returnvalue (Abilities|TryActivateAbilitybyClass (Variables|Default|GetAbilitySystem) "/Game/MyContent/Blueprints/GameplayAbility/GA_NormalAttack.GA_NormalAttack_C" false))
    (if _returnvalue
      (CallFunction|AutoTarget)
      (elif (Variables|/Script/MirrorOfShadows.PlayerCore|GetCanBuffer _charactercore)
        (if (not (Variables|/Script/MirrorOfShadows.PlayerCore|GetHasBuffer _charactercore))
          (Variables|/Script/MirrorOfShadows.PlayerCore|SetHasBuffer _charactercore true)
          (Development|PrintString "Created Buffer"))))))

(event Input|EnhancedActionEvents|EnhancedInputActionIA_Skill1
  (params (ActionValue :type Boolean) (ElapsedSeconds :type Float%20%28double-precision%29) (TriggeredSeconds :type Float%20%28double-precision%29) (InputAction :type Input%20Action%20Object%20Reference :default "/Game/MyContent/InputActions/IA_Skill1.IA_Skill1"))
  (bind _skilldata (Variables|Default|GetSkillData))
  (:Started
    (Development|PrintString "Calling SKill")
    (if (> (Utilities|Array|Length _skilldata) 0)
      (if (Utilities|Array|IsValidIndex _skilldata)
        (Variables|Default|SetActiveSkill (Utilities|Array|Get(acopy) _skilldata))
        (bind _returnvalue (Abilities|TryActivateAbilitybyClass (Variables|Default|GetAbilitySystem) "/Game/MyContent/Blueprints/GameplayAbility/GA_GenericPlayerSkill.GA_GenericPlayerSkill_C" false))
        (if _returnvalue
          (Development|PrintString "Skill Activate")
          (else
            (Development|PrintString "Skill Didn't activate")))
        (else
          (Development|PrintString "Fail2")))
      (else
        (Development|PrintString "Fail")))))

(event EventBeginPlay
  (bind _abilitysystem (Variables|Default|GetAbilitySystem))
  (GameplayAbilities|GiveAbility _abilitysystem "/Game/MyContent/Blueprints/GameplayAbility/GA_NormalAttack.GA_NormalAttack_C" 0 -1)
  (GameplayAbilities|GiveAbility _abilitysystem "/Game/MyContent/Blueprints/GameplayAbility/GA_GenericPlayerSkill.GA_GenericPlayerSkill_C" 0 0)
  (if (> (Utilities|Array|Length (Variables|/Script/MirrorOfShadows.EquipmentComponent|GetEquippedGear (Variables|Default|GetEquipmentComponent))) 0)
    (CallFunction|ApplyGearStats)))

(event Collision|EventActorBeginOverlap
  (params (OtherActor :type Actor%20Object%20Reference)))

(event Game|Damage|EventAnyDamage
  (params (Damage :type Float%20%28single-precision%29) (DamageType :type Damage%20Type%20Object%20Reference) (InstigatedBy :type Controller%20Object%20Reference) (DamageCauser :type Actor%20Object%20Reference))
  (Game|SpawnActorfromClass "/Game/MyContent/Blueprints/UI/CombatUI/BP_DamageNumber.BP_DamageNumber_C" (Transformation|GetActorTransform) "Undefined" "MultiplyWithRoot" 0 Damage (Transformation|GetActorLocation) 0))

(event EventTick
  (params (DeltaSeconds :type Float%20%28single-precision%29))
  (Variables|Default|SetOnGround (AI|Components|NavMovement|IsMovingonGround (Variables|Character|GetCharacterMovement))))

(event EventEndHitStop
  (Variables|Default|SetCustomTimeDilation 1.0)
  (for _array_element (Variables|Default|GetVFXList)
    (Utilities|IsValid _array_element
      (:Is%20Valid
        (Class|NiagaraComponent|SetCustomTimeDilation _array_element 1.0)))))

(event EventStartHitStop
  (Variables|Default|SetCustomTimeDilation 0.1)
  (Utilities|Time|SetTimerbyFunctionName 0 "EndHitStop" 0.1)
  (for _array_element (Variables|Default|GetVFXList)
    (Utilities|IsValid _array_element
      (:Is%20Valid
        (Class|NiagaraComponent|SetCustomTimeDilation _array_element 0.1)))))

(event EventDestroyed)

(event EventPossessed
  (params (NewController :type Controller%20Object%20Reference)))

(event EventNormalAttackAbility
  (bind _charactercore (Variables|Default|GetCharacterCore))
  (bind _returnvalue (Abilities|TryActivateAbilitybyClass (Variables|Default|GetAbilitySystem) "/Game/MyContent/Blueprints/GameplayAbility/GA_NormalAttack.GA_NormalAttack_C" false))
  (if _returnvalue
    (CallFunction|AutoTarget)
    (elif (Variables|/Script/MirrorOfShadows.PlayerCore|GetCanBuffer _charactercore)
      (if (not (Variables|/Script/MirrorOfShadows.PlayerCore|GetHasBuffer _charactercore))
        (Variables|/Script/MirrorOfShadows.PlayerCore|SetHasBuffer _charactercore true)
        (Development|PrintString "Created Buffer")))))

(event Input|KeyboardEvents|DebugKeyP
  (params (Key :type Key%20Structure :default "None") (ActionValue :type Input%20Action%20Value%20Structure))
  (:Released
    (bind _returnvalue (GameplayEffects|RemoveActiveEffectswithGrantedTags (Variables|Default|GetAbilitySystem) "(GameplayTags=((TagName=\"Equipment.Armor.Helmet\")))"))
    (Development|PrintString (Utilities|String|Append "Removed " (Utilities|String|ToString(Integer) _returnvalue) " effects"))))

(fn ConstructionScript)

(fn SummonEffect
  (params (ParticleTransform :type Transform) (VFX :type Niagara%20System%20Object%20Reference))
  (bind _slashspot (Variables|Default|GetSlashSpot))
  (bind _returnvalue (Transformation|GetWorldTransform _slashspot))
  (Transformation|SetRelativeTransform _slashspot ParticleTransform false false)
  (bind _returnvalue_2 (Niagara|SpawnSystematLocation VFX (.location _returnvalue) (.rotation _returnvalue) (.scale _returnvalue)))
  (Utilities|Array|Add (Variables|Default|GetVFXList) _returnvalue_2))

(fn DestroyEffects
  (Utilities|Array|Clear (Variables|Default|GetVFXList)))

(fn ApplyGearStats
  (for _array_element (Variables|/Script/MirrorOfShadows.EquipmentComponent|GetEquippedGear (Variables|Default|GetEquipmentComponent))
    (Utilities|IsValid _array_element
      (:Is%20Valid
        (|SwitchGameplayTag (Variables|/Script/MirrorOfShadows.Armor|GetEquipSlot _array_element)
          (:Equipment.Armor.Helmet
            (CallFunction|TurnStatsintoEffect "/Game/MyContent/Blueprints/GameplayEffect/ArmorSlotEffects/GE_HelmetStats.GE_HelmetStats_C" (Variables|/Script/MirrorOfShadows.Equipment|GetSubStats _array_element) (Variables|/Script/MirrorOfShadows.Equipment|GetMainStat _array_element) (Variables|/Script/MirrorOfShadows.Equipment|GetMainStatValue _array_element))))))))

(fn TurnStatsintoEffect
  (params (EquipmentClass :type Gameplay%20Effect%20Class%20Reference) (SubStatMap :type Map%20of%20Gameplay%20Tag%20Structures%20to%20Reals) (MainStatTag :type Gameplay%20Tag%20Structure) (MainStatValue :type Float%20%28double-precision%29))
  (bind _abilitysystem (Variables|Default|GetAbilitySystem))
  (LocalVariables|SetEffectSpec (GameplayEffects|MakeOutgoingSpec :self (Variables|Default|GetAbilitySystem) :GameplayEffectClass EquipmentClass))
  (|SwitchGameplayTag MainStatTag
    (:Default
      _)
    (:Stats.Flat.HP
      (Ability|GameplayEffect|AssignTagSetbyCallerMagnitude (LocalVariables|GetEffectSpec) MainStatTag MainStatValue)
      (Development|PrintString (Utilities|String|Append "Adding in " (Utilities|String|ToString(Float) MainStatValue) "HP to max"))))
  (for _array_element (LocalVariables|GetStatTags)
    (if (.ReturnValue (Utilities|Map|Find SubStatMap _array_element))
      (Ability|GameplayEffect|AssignTagSetbyCallerMagnitude (LocalVariables|GetEffectSpec) _array_element (.Value (Utilities|Map|Find SubStatMap _array_element)))
      (else
        (Ability|GameplayEffect|AssignTagSetbyCallerMagnitude (LocalVariables|GetEffectSpec) _array_element 0.0))))
  (GameplayEffects|ApplyGameplayEffectSpecToSelf _abilitysystem (LocalVariables|GetEffectSpec))
  (GameplayEffects|ApplyGameplayEffectToSelf :self _abilitysystem :GameplayEffectClass "/Game/MyContent/Blueprints/GameplayEffect/GE_SetCurHP.GE_SetCurHP_C"))

(fn AutoTarget
  (bind _returnvalue (Transformation|GetActorRotation))
  (bind _lockontarget (Variables|Default|GetLockOnTarget))
  (if (and (Variables|Default|GetHasLockOn) (Utilities|IsValid _lockontarget))
    (Transformation|SetActorRotation (Math|Rotator|MakeRotator (.roll _returnvalue) (.pitch _returnvalue) (.yaw (Math|Rotator|FindLookatRotation (Transformation|GetActorLocation) (Transformation|GetActorLocation _lockontarget)))))))