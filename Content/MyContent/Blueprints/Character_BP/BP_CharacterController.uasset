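; Player controller that handles enemy lock-on targeting and left character swapping between summoned characters.
; A debug Tab key toggles lock-on, using a sphere trace to pick the nearest Enemy-tagged actor and passing it to the current character.
; While locked, Tick interpolates control rotation toward the target.
; Swapping cancels montages and normal-attack effects, switches character, then notifies the current player state object.
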(event Custom|SetUpState
  (params (PlayerState :type BP%20Player%20State%20Object%20Reference))
  (Variables|Default|SetCurrentState PlayerState))

(event Input|EnhancedActionEvents|EnhancedInputActionIA_LeftCharacterSwap
  (params (ActionValue :type Boolean) (ElapsedSeconds :type Float%20%28double-precision%29) (TriggeredSeconds :type Float%20%28double-precision%29) (InputAction :type Input%20Action%20Object%20Reference :default "/Game/MyContent/InputActions/IA_LeftCharacterSwap.IA_LeftCharacterSwap"))
  (bind _returnvalue (Game|GetPlayerCharacter 0))
  (:Started
    (Animation|StopAnimMontage _returnvalue 0)
    (GameplayEffects|RemoveActiveEffectswithGrantedTags (Ability|GetAbilitySystemComponent _returnvalue) "(GameplayTags=((TagName=\"Ability.Input.NormalAttack\"),(TagName=\"Ability.Input.Skill\")))")
    (Class|PlayerPartyController|SwapCharacterLeft)
    (Default|OnSwap (Variables|Default|GetCurrentState) (Variables|Default|GetActiveCharacter))
    (Class|PlayerPartyController|SwitchResponse)))

(event EventTick
  (params (DeltaSeconds :type Float%20%28single-precision%29))
  (if (Variables|Default|GetIsLockedOn)
    (CallFunction|LockonCamera)))

(event Input|KeyboardEvents|DebugKeyTab
  (params (Key :type Key%20Structure :default "None") (ActionValue :type Input%20Action%20Value%20Structure))
  (:Pressed
    (if (Variables|Default|GetIsLockedOn)
      (bind _output_get (Variables|Default|SetIsLockedOn false))
      (Class|PlayerCharacters|SetUpLockon (Utilities|Array|Get(acopy) (Variables|Default|GetSummonedActorReferences) (Variables|Default|GetCurrentCharacter)) _output_get)
      (else
        (CallFunction|StartLockon)))))

(fn ConstructionScript)

(fn StartLockon
  (bind _returnvalue (Game|GetPlayerCharacter 0))
  (bind _trackedactors (LocalVariables|GetTrackedActors))
  (bind _returnvalue_2 (Transformation|GetActorLocation _returnvalue))
  (bind _outhits (Collision|MultiSphereTraceByChannel _returnvalue_2 (* _returnvalue_2 (* (Math|Vector|GetForwardVector (Variables|/Script/Engine.PlayerCameraManager|GetTransformComponent (Game|GetPlayerCameraManager 0))) (LocalVariables|GetMinDist))) 1e+02 "TraceTypeQuery4" false (Utilities|Array|MakeArray _returnvalue) "ForDuration"))
  (for _array_element _outhits
    (if (not (Utilities|Array|ContainsItem _trackedactors (.HitActor (Collision|BreakHitResult _array_element))))
      (Utilities|Array|Add _trackedactors (.HitActor (Collision|BreakHitResult _array_element)))
      (if (Actor|ActorHasTag (.HitActor (Collision|BreakHitResult _array_element)) "Enemy")
        (if (< (Math|Vector|Distance(Vector) (.Location (Collision|BreakHitResult _array_element)) _returnvalue_2) (LocalVariables|GetMinDist))
          (LocalVariables|SetMinDist (Math|Vector|Distance(Vector) (.Location (Collision|BreakHitResult _array_element)) _returnvalue_2))
          (Variables|Default|SetLockOnTarget (.HitActor (Collision|BreakHitResult _array_element)))
          (Variables|Default|SetIsLockedOn true)))))
  (if (Variables|Default|GetIsLockedOn)
    (Class|PlayerCharacters|SetUpLockon (Utilities|Array|Get(acopy) (Variables|Default|GetSummonedActorReferences) (Variables|Default|GetCurrentCharacter)) (Variables|Default|GetIsLockedOn) (Variables|Default|GetLockOnTarget))))

(fn LockonCamera
  (bind _returnvalue (Game|GetPlayerCharacter 0))
  (bind _returnvalue_2 (Transformation|GetActorRotation))
  (bind _returnvalue_3 (Utilities|Time|GetWorldDeltaSeconds))
  (bind _lockontarget (Variables|Default|GetLockOnTarget))
  (bind _returnvalue_4 (Transformation|GetActorLocation _lockontarget))
  (bind _returnvalue_5 (Transformation|GetActorLocation _returnvalue))
  (bind _returnvalue_6 (- (.z _returnvalue_4) 1.5e+02))
  (bind _returnvalue_7 (Math|Rotator|FindLookatRotation _returnvalue_5 (Math|Vector|MakeVector (.x _returnvalue_4) (.y _returnvalue_4) _returnvalue_6)))
  (bind _returnvalue_8 (Math|Interpolation|RInterpTo _returnvalue_2 _returnvalue_7 _returnvalue_3 5.0))
  (Pawn|SetControlRotation (Math|Rotator|MakeRotator (.Roll (Math|Rotator|BreakRotator _returnvalue_2)) (.pitch _returnvalue_8) (.yaw _returnvalue_8))))