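; Anim notify state that yaws a BP_EnemyBase owner relative to its AttackTarget while the notify window is active.
; Each tick adds world yaw equal to actor yaw minus look-at yaw, scaled by delta time and RotationSpeed, without angle normalization.
; On end, it prints a debug check of whether the AI controller's control rotation differs from the actor's rotation.
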(fn `Received_NotifyEnd`
  (params (MeshComp :type "SkeletalMeshComponent Object Reference") (Animation :type "AnimSequenceBase Object Reference") (EventReference :type "AnimNotifyEventReference Structure (by ref)"))
  (returns (ReturnValue :type Boolean))
  (bind _returnvalue (`ActorComponent.GetOwner` MeshComp))
  (`KismetSystemLibrary.PrintString` null (`KismetStringLibrary.Conv_BoolToString` (!= (`Controller.GetControlRotation` (`AIBlueprintHelperLibrary.GetAIController` _returnvalue)) (`Actor.K2_GetActorRotation` _returnvalue) :`ErrorTolerance` 0.1)))
  (return false))

(fn `Received_NotifyTick`
  (params (MeshComp :type "SkeletalMeshComponent Object Reference") (Animation :type "AnimSequenceBase Object Reference") (FrameDeltaTime :type "Float (single-precision)") (EventReference :type "AnimNotifyEventReference Structure (by ref)"))
  (returns (ReturnValue :type Boolean))
  (bind _asbp_enemy_base (cast `/Game/MyContent/Blueprints/Enemy_BP/BP_EnemyBase` (`ActorComponent.GetOwner` MeshComp)))
  (bind (_returnvalue_roll _returnvalue_pitch _returnvalue_yaw) (`KismetMathLibrary.BreakRotator` (`Actor.K2_GetActorRotation` _asbp_enemy_base)))
  (bind (_returnvalue_roll_2 _returnvalue_pitch_2 _returnvalue_yaw_2) (`KismetMathLibrary.BreakRotator` (`KismetMathLibrary.FindLookAtRotation` (`Actor.K2_GetActorLocation` _asbp_enemy_base) (`Actor.K2_GetActorLocation` (`EnemyCharacterBase.AttackTarget` _asbp_enemy_base)))))
  (`Actor.K2_AddActorWorldRotation` _asbp_enemy_base (`KismetMathLibrary.MakeRotator` 0.0 0.0 (* (- _returnvalue_yaw _returnvalue_yaw_2) FrameDeltaTime (`self.RotationSpeed`))) false false)
  (return false))