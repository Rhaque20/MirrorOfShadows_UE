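; Anim notify state that marks the recovery window of a player skill attack animation.
; On begin it puts the player's CharacterCore into recovery, resets the combo chain, clears the skill input tag's effects, sends a melee recover gameplay event and re-enables movement.
; On end it clears normal-attack input effects if the player is no longer attacking, then destroys the player's effects.
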(fn `Received_NotifyBegin`
  (params (MeshComp :type "SkeletalMeshComponent Object Reference") (Animation :type "AnimSequenceBase Object Reference") (TotalDuration :type "Float (single-precision)") (EventReference :type "AnimNotifyEventReference Structure (by ref)"))
  (returns (ReturnValue :type Boolean))
  (locals (BufferReact :type Boolean))
  (bind _returnvalue (`ActorComponent.GetOwner` MeshComp))
  (bind _asbp_player (cast `/Game/MyContent/Blueprints/Character_BP/BP_Player` _returnvalue))
  (bind _charactercore (`CecilePlayable.CharacterCore` _asbp_player))
  (`PlayerCore.Recover` _charactercore)
  (set `PlayerCore.CurrentChain` 0 _charactercore)
  (`AbilitySystemComponent.RemoveActiveEffectsWithGrantedTags` (`AbilitySystemBlueprintLibrary.GetAbilitySystemComponent` _returnvalue) (struct :`GameplayTags` (struct :`(TagName` "Ability.Input.Skill"))))
  (`AbilitySystemBlueprintLibrary.SendGameplayEventToActor` _returnvalue (struct :`TagName` "Event.Melee.Recover"))
  (`KismetSystemLibrary.PrintString` MeshComp "In Recovery State")
  (set `PlayerCharacters.CanMove` true _asbp_player)
  (return false))

(fn `Received_NotifyEnd`
  (params (MeshComp :type "SkeletalMeshComponent Object Reference") (Animation :type "AnimSequenceBase Object Reference") (EventReference :type "AnimNotifyEventReference Structure (by ref)"))
  (returns (ReturnValue :type Boolean))
  (bind _returnvalue (`ActorComponent.GetOwner` MeshComp))
  (bind _asbp_player (cast `/Game/MyContent/Blueprints/Character_BP/BP_Player` _returnvalue))
  (if (not (`CombatComponent.bIsAttacking` (`PlayerCharacters.CharacterCore` _asbp_player)))
    (`AbilitySystemComponent.RemoveActiveEffectsWithGrantedTags` (`AbilitySystemBlueprintLibrary.GetAbilitySystemComponent` _returnvalue) (struct :`GameplayTags` (struct :`(TagName` "Ability.Input.NormalAttack")))))
  (`/Game/MyContent/Blueprints/Character_BP/BP_Player.DestroyEffects` _asbp_player)
  (`KismetSystemLibrary.PrintString` null "End Skill Notify")
  (return false))