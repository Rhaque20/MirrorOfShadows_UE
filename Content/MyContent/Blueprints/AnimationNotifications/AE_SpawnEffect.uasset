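; AE_SpawnEffect is an animation notify that has the player spawn a visual effect from within an animation.
; It casts the mesh owner to BP_Player and calls its SummonEffect with the configured VFX and ParticleTransform, doing nothing for other owners.
; When OverrideTransform is set, it replaces the transform's rotation with ParticleRotation while keeping location and scale.
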(fn `Received_Notify`
  (params (MeshComp :type "SkeletalMeshComponent Object Reference") (Animation :type "AnimSequenceBase Object Reference") (EventReference :type "AnimNotifyEventReference Structure (by ref)"))
  (returns (ReturnValue :type Boolean))
  (bind _vfx (`self.VFX`))
  (bind (_particletransform_location _particletransform_rotation _particletransform_scale) (`KismetMathLibrary.BreakTransform` (`self.ParticleTransform`)))
  (bind _asbp_player (cast `/Game/MyContent/Blueprints/Character_BP/BP_Player` (`ActorComponent.GetOwner` MeshComp)))
  (if (`self.OverrideTransform`)
    (`/Game/MyContent/Blueprints/Character_BP/BP_Player.SummonEffect` _asbp_player (`KismetMathLibrary.MakeTransform` _particletransform_location (`self.ParticleRotation`) _particletransform_scale) _vfx)
    (else
      (`/Game/MyContent/Blueprints/Character_BP/BP_Player.SummonEffect` _asbp_player (`self.ParticleTransform`) _vfx)))
  (return false))