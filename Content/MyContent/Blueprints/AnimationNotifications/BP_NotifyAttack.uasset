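; Anim notify state that marks the recovery window of the player's attack animations and drives combo chaining.
; On begin it stops the launch timeline, calls Recover on CharacterCore, removes normal-attack input effects and sends the melee recover gameplay event.
; A buffered input then triggers the next normal attack; otherwise movement is allowed unless an aerial action is running.
; On end it updates attack and chain state and destroys the player's effects.
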(fn `Received_NotifyBegin`
  (params (MeshComp :type "SkeletalMeshComponent Object Reference") (Animation :type "AnimSequenceBase Object Reference") (TotalDuration :type "Float (single-precision)") (EventReference :type "AnimNotifyEventReference Structure (by ref)"))
  (returns (ReturnValue :type Boolean))
  (locals (BufferReact :type Boolean) (PlayerRef :type "/Game/MyContent/Blueprints/Character_BP/BP_Player Object Reference"))
  (bind _returnvalue (`ActorComponent.GetOwner` MeshComp))
  (bind _playerref (`local.PlayerRef`))
  (bind _charactercore (`CecilePlayable.CharacterCore` (`local.PlayerRef`)))
  (bind _hasbuffer (`PlayerCore.HasBuffer` _charactercore))
  (bind _asbp_player (cast `/Game/MyContent/Blueprints/Character_BP/BP_Player` _returnvalue))
  (bind _output_get (set `local.PlayerRef` _asbp_player))
  (`RPGCharacterBase.StopLaunchTimeLine` _output_get)
  (if _hasbuffer
    (bind _output_get_2 (set `local.BufferReact` _hasbuffer)))
  (`PlayerCore.Recover` _charactercore)
  (`AbilitySystemComponent.RemoveActiveEffectsWithTags` (`AbilitySystemBlueprintLibrary.GetAbilitySystemComponent` _returnvalue) (struct :`GameplayTags` (struct :`(TagName` "Ability.Input.NormalAttack"))))
  (`AbilitySystemBlueprintLibrary.SendGameplayEventToActor` _returnvalue (struct :`TagName` "Event.Melee.Recover"))
  (if _output_get_2
    (`PlayerCharacters.NormalAttackAbility` _playerref)
    (else
      (set `PlayerCharacters.CanMove` (not (`PlayerCharacters.bIsPerformingAerialAction` (`local.PlayerRef`))) _playerref)))
  (return false))

(fn `Received_NotifyEnd`
  (params (MeshComp :type "SkeletalMeshComponent Object Reference") (Animation :type "AnimSequenceBase Object Reference") (EventReference :type "AnimNotifyEventReference Structure (by ref)"))
  (returns (ReturnValue :type Boolean))
  (bind _asbp_player (cast `/Game/MyContent/Blueprints/Character_BP/BP_Player` (`ActorComponent.GetOwner` MeshComp)))
  (bind _charactercore (`CecilePlayable.CharacterCore` _asbp_player))
  (if (`CombatComponent.bIsAttacking` _charactercore)
    (if (`PlayerCore.EndOfChain` _charactercore)
      (set `CombatComponent.bIsAttacking` false _charactercore))
    (else
      (set `PlayerCore.CurrentChain` 0 _charactercore)))
  (`/Game/MyContent/Blueprints/Character_BP/BP_Player.DestroyEffects` _asbp_player)
  (return false))