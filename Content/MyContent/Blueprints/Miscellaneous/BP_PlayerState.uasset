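; BP_PlayerState tracks the active player character across swaps and runs the evade slow-motion counter window.
; BeginPlay and OnSwap store the active BP_Player and give it a back-reference, and BeginPlay also registers the state with BP_CharacterController.
; TriggerEvadeSlowDown drives global time dilation through a timeline while a counter is allowed.
; When it finishes, a flagged counter makes the character normal-attack the evaded target.
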(event `OnSwap`
  (params (NewCharacter :type "PlayerCharacters Object Reference"))
  (bind _asbp_player (cast `/Game/MyContent/Blueprints/Character_BP/BP_Player` NewCharacter))
  (bind _output_get (set `self.ActiveCharacter` _asbp_player))
  (set `/Game/MyContent/Blueprints/Character_BP/BP_Player.PlayerStateRef` self _output_get)
  (`KismetSystemLibrary.PrintString` "Set up state"))

(event `self.ReceiveBeginPlay`
  (bind _asbp_character_controller (cast `/Game/MyContent/Blueprints/Character_BP/BP_CharacterController` (`self.GetPlayerController`)))
  (bind _asbp_player (cast `/Game/MyContent/Blueprints/Character_BP/BP_Player` (`PlayerPartyController.ActiveCharacter` _asbp_character_controller)))
  (bind _output_get (set `self.ActiveCharacter` _asbp_player))
  (set `/Game/MyContent/Blueprints/Character_BP/BP_Player.PlayerStateRef` self _output_get)
  (`/Game/MyContent/Blueprints/Character_BP/BP_CharacterController.SetUpState` _asbp_character_controller self))

(event `TriggerEvadeSlowDown`
  (params (CounteredTarget :type "/Game/MyContent/Blueprints/Enemy_BP/BP_EnemyBase Object Reference"))
  (bind _activecharacter (`self.ActiveCharacter`))
  (if (not (`TimelineComponent.IsPlaying` (`self.EvasionSlowMotion`)))
    (set `self.Countered Target` CounteredTarget)
    (set `self.CanCounterEdge` true)
    (bind (_direction _timedilationscale) (`Timeline|EvasionSlowMotion` :!via `PlayFromStart`)
      (:`Update`
        (`GameplayStatics.SetGlobalTimeDilation` _timedilationscale))
      (:`Finished`
        (`KismetSystemLibrary.PrintString` "Player State Slow Mo End")
        (set `self.CanCounterEdge` false)
        (if (`self.ActivateCounterEdge`)
          (set `/Game/MyContent/Blueprints/Character_BP/BP_Player.CounterTarget` (`self.Countered Target`) _activecharacter)
          (set `self.ActivateCounterEdge` false)
          (`PlayerCharacters.NormalAttackAbility` _activecharacter))
        (set `self.Countered Target` null)))))

(fn `InitiateCounterEdge`
  (returns (CounterTarget :type "/Game/MyContent/Blueprints/Enemy_BP/BP_EnemyBase Object Reference"))
  (return (`self.Countered Target`)))

(fn `UserConstructionScript`)