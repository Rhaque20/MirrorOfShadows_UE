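; Enemy stagger component that handles hit reactions, interrupts and stance breaks for BP_EnemyBase owners.
; Interrupts and stance breaks share a timer that halts montage, attack and movement, then calls Recover and sends a gameplay event.
; Stance breaks last longer and apply GE_StanceBroken with a SetByCaller duration.
; Hits either trigger a Blackboard dodge through an evade-cooldown tag query or run parent handling and put the enemy in combat.
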(event `self.InterruptRecover`
  (`EnemyCharacterBase.Recover` (`self.EnemyOwner`))
  (`KismetSystemLibrary.PrintString` "Stagger Time End")
  (set `self.ActivatedStanceTimer` false)
  (`AbilitySystemBlueprintLibrary.SendGameplayEventToActor` (`self.GetOwner`) (struct :`TagName` "Event.Melee.Recover"))
  (`KismetSystemLibrary.PrintString` "Move Recov Stag"))

(event `self.OnStanceBreak`
  (bind _staggertimer (`self.StaggerTimer`))
  (if (not (`self.ActivatedStanceTimer`))
    (`KismetSystemLibrary.PrintString` "Stance Timer Begin")
    (set `self.ActivatedStanceTimer` true)
    (bind _output_get (set `self.StaggerDuration` 3.0))
    (if (`KismetSystemLibrary.K2_IsTimerActiveHandle` _staggertimer)
      (`KismetSystemLibrary.K2_ClearAndInvalidateTimerHandle` _staggertimer))
    (bind _returnvalue (`AbilitySystemBlueprintLibrary.AssignTagSetByCallerMagnitude` (`AbilitySystemComponent.MakeOutgoingSpec` :`self` (`self.AbilitySystemComponent`) :`GameplayEffectClass` "/Game/MyContent/Blueprints/GameplayEffect/StanceSystem/GE_StanceBroken.GE_StanceBroken_C") (struct :`TagName` "Effect.State.StanceBroken") _output_get))
    (`AbilitySystemComponent.BP_ApplyGameplayEffectSpecToSelf` (`self.AbilitySystemComponent`) _returnvalue)
    (`self.Interruption Timer ` (delegate `self.InterruptRecover`))
    (set `RPGCharacterBase.CanMove` false (`self.EnemyOwner`))))

(event `self.OnInterrupt`
  (bind _staggertimer (`self.StaggerTimer`))
  (`parent.OnInterrupt`)
  (if (and (`KismetSystemLibrary.K2_IsTimerActiveHandle` _staggertimer) (not (`GameplayTagAssetInterface.HasMatchingGameplayTag` (`self.AbilitySystemComponent`) (struct :`TagName` "Effect.State.StanceBroken"))))
    (`KismetSystemLibrary.K2_ClearAndInvalidateTimerHandle` _staggertimer))
  (set `self.StaggerDuration` 1.5)
  (set `RPGCharacterBase.CanMove` false (`self.EnemyOwner`))
  (`self.Interruption Timer ` (delegate `self.InterruptRecover`)))

(event `self.ReceiveBeginPlay`
  (`parent.ReceiveBeginPlay`)
  (bind _asbp_enemy_base (cast `/Game/MyContent/Blueprints/Enemy_BP/BP_EnemyBase` (`self.GetOwner`)))
  (set `self.EnemyOwner` _asbp_enemy_base))

(fn `HasDetectedPlayer`
  (bind _enemyowner (`self.EnemyOwner`))
  (bind _returnvalue (`AIBlueprintHelperLibrary.GetBlackboard` _enemyowner))
  (if (not (`/Game/MyContent/Blueprints/Enemy_BP/BP_EnemyBase.SpotsPlayer` _enemyowner))
    (bind _output_get (set `/Game/MyContent/Blueprints/Enemy_BP/BP_EnemyBase.SpotsPlayer` true _enemyowner))
    (`BlackboardComponent.SetValueAsBool` _returnvalue "InCombat" _output_get)
    (`BlackboardComponent.SetValueAsObject` _returnvalue "Target" (`GameplayStatics.GetPlayerPawn` 0))))

(fn `Interruption Timer `
  (params (Delegate :type Delegate))
  (returns (EnemyOwner :type "/Game/MyContent/Blueprints/Enemy_BP/BP_EnemyBase Object Reference"))
  (bind _enemyowner (`self.EnemyOwner`))
  (`Character.StopAnimMontage` _enemyowner null)
  (set `EnemyCharacterBase.CanMove` false _enemyowner)
  (set `EnemyCharacterBase.IsAttacking` false _enemyowner)
  (bind _returnvalue (`KismetSystemLibrary.K2_SetTimerDelegate` Delegate (`self.StaggerDuration`)))
  (set `self.StaggerTimer` _returnvalue)
  (return _enemyowner))

(fn `OnHit`
  (returns (HitResult :type Boolean))
  (if (and (`BlueprintGameplayTagLibrary.DoesContainerMatchTagQuery` (`GameplayTagAssetInterface.GetOwnedGameplayTags` (`AbilitySystemBlueprintLibrary.GetAbilitySystemComponent` (`self.EnemyOwner`))) (`BlueprintGameplayTagLibrary.MakeGameplayTagQuery` (struct :`TagDictionary` (struct :`(TagName` "Skill.Cooldown.Evade") :`(TagName` "Ability.Input.NormalAttack") :`(TagName` "Effect.State.PoiseBroken") :`(TagName` "Effect.State.StanceBroken")) :`QueryTokenStream` "(0,1,5,2,1,1,0,3,3,1,2,3)" :`AutoDescription` " ALL(  ANY( Skill.Cooldown.Evade ),  NONE( Ability.Input.NormalAttack, Effect.State.PoiseBroken, Effect.State.StanceBroken ) )"))) (`/Game/MyContent/Blueprints/Enemy_BP/BP_EnemyBase.SpotsPlayer` (`self.EnemyOwner`)))
    (`BlackboardComponent.SetValueAsBool` (`AIBlueprintHelperLibrary.GetBlackboard` (`self.EnemyOwner`)) "TriggerDodge" true)
    (return false)
    (else
      (bind _hitresult (`parent.OnHit`))
      (`self.HasDetectedPlayer`)
      (return _hitresult))))