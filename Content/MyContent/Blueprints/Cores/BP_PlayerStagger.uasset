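; BP_PlayerStagger is the player's stagger component, handling interrupt, parry and hit responses for its BP_Player owner.
; An interrupt stops the montage, blocks movement and dodging, and restarts a timer that calls PlayerRecover.
; A parry activates a dodge and clears the parry cooldown by removing tagged gameplay effects.
; OnHit defers to the parent and returns true, while PerfectDodgeTest is empty, with its iframe-refresh logic disconnected.
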(event `self.ReceiveBeginPlay`
  (`parent.ReceiveBeginPlay`)
  (bind _asbp_player (cast `/Game/MyContent/Blueprints/Character_BP/BP_Player` (`self.GetOwner`)))
  (set `self.PlayerOwner` _asbp_player))

(event `self.OnInterrupt`
  (bind _playerowner (`self.PlayerOwner`))
  (bind _staggertimer (`self.StaggerTimer`))
  (if (`KismetSystemLibrary.K2_IsTimerActiveHandle` _staggertimer)
    (`KismetSystemLibrary.K2_ClearAndInvalidateTimerHandle` _staggertimer))
  (`Character.StopAnimMontage` _playerowner null)
  (bind _returnvalue (`KismetSystemLibrary.K2_SetTimerDelegate` (delegate `self.InterruptRecover`) 1.5))
  (set `self.StaggerTimer` _returnvalue)
  (set `PlayerCharacters.CanMove` false _playerowner)
  (set `/Game/MyContent/Blueprints/Character_BP/BP_Player.CanDodge` false _playerowner)
  (`KismetSystemLibrary.PrintString` "Player Interrupt!"))

(event `self.InterruptRecover`
  (`PlayerCharacters.PlayerRecover` (`self.PlayerOwner`)))

(fn `OnHit`
  (returns (HitResult :type Boolean))
  (`parent.OnHit`)
  (return true))

(fn `OnParry`
  (`/Game/MyContent/Blueprints/Character_BP/BP_Player.ActivateDodge` (`self.PlayerOwner`))
  (`AbilitySystemComponent.RemoveActiveEffectsWithGrantedTags` (`self.AbilitySystemComponent`) (struct :`GameplayTags` (struct :`(TagName` "Skill.Cooldown.Parry"))))
  (return))

(fn `PerfectDodgeTest`)