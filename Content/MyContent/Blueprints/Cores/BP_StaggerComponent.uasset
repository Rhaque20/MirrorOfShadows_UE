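; Stagger component that uses the owner's Ability System Component, cached on BeginPlay, to react to poise and stance breaks.
; A poise break on a living owner applies GE_PoiseBroken if not already broken, tries the hit reaction ability and disables RPGCharacterBase movement.
; Stance break only prints and calls OnInterrupt, which is a stub, as are interrupt recovery and the interruption timer.
; OnHit calls the parent and returns true.
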(event `self.OnInterrupt`
  (cast `Character` (`self.GetOwner`)))

(event `self.OnStanceBreak`
  (`KismetSystemLibrary.PrintString` "StanceBroken")
  (`self.OnInterrupt`))

(event `InterruptRecover`)

(event `self.ReceiveBeginPlay`
  (set `self.AbilitySystemComponent` (`AbilitySystemBlueprintLibrary.GetAbilitySystemComponent` (`self.GetOwner`))))

(event `self.OnPoiseBreak`
  (bind _abilitysystemcomponent (`self.AbilitySystemComponent`))
  (`/Engine/EditorBlueprintResources/StandardMacros.IsValid` _abilitysystemcomponent
    (:`Is Valid`
      (if (not (`GameplayTagAssetInterface.HasMatchingGameplayTag` _abilitysystemcomponent (struct :`TagName` "Effect.State.Dead")))
        (if (not (`GameplayTagAssetInterface.HasMatchingGameplayTag` _abilitysystemcomponent (struct :`TagName` "Effect.State.PoiseBroken")))
          (`AbilitySystemComponent.BP_ApplyGameplayEffectToSelf` :`self` _abilitysystemcomponent :`GameplayEffectClass` "/Game/MyContent/Blueprints/GameplayEffect/PoiseSystem/GE_PoiseBroken.GE_PoiseBroken_C"))
        (`self.OnInterrupt`)
        (`AbilitySystemComponent.TryActivateAbilityByClass` (`self.AbilitySystemComponent`) (`self.HitReactionAbility`) true)
        (bind _asrpgcharacter_base (cast `RPGCharacterBase` (`self.GetOwner`)))
        (set `RPGCharacterBase.CanMove` false _asrpgcharacter_base)))))

(fn `Interruption Timer `
  (params (Delegate :type "Object Object Reference"))
  (returns (EnemyOwner :type "/Game/MyContent/Blueprints/Enemy_BP/BP_EnemyBase Object Reference"))
  (return null))

(fn `OnHit`
  (returns (HitResult :type Boolean))
  (`parent.OnHit`)
  (return true))